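; Player character for a three-lane runner that switches lanes, jumps and drops fast, with a HUD and pause key.
; Tick detects one swipe per touch past a distance threshold; keyboard and action inputs share the same movement branches.
; A timeline lerps Y between lane positions, while a downward impulse handles lowering.
; DeathFunction ragdolls the mesh, shows game over and saves the game mode's points if they beat the stored high score.
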(event `Key|Tab` :paused true
  (params (Key :type "Key Structure"))
  (:`Pressed`
    (`GameplayStatics.SetGamePaused` true)))

(event `self.ReceiveBeginPlay`
  (bind _returnvalue (`|CreateWidget` "/Game/UI/HUD/WBP_HUD.WBP_HUD_C"))
  (bind _output_get (set `self.HUD` _returnvalue))
  (`UserWidget.AddToViewport` _output_get 0))

(event `self.ReceiveTick`
  (params (DeltaSeconds :type "Float (single-precision)"))
  (bind _laney (`self.LaneY`))
  (bind (_locationx _locationy) (`PlayerController.GetInputTouchState` (`GameplayStatics.GetPlayerController` 0) "Touch1"))
  (bind (_returnvalue_x _returnvalue_y _returnvalue_z) (`KismetMathLibrary.BreakVector` (`SceneComponent.K2_GetComponentLocation` (`self.CapsuleComponent`))))
  (bind _returnvalue (`KismetMathLibrary.MakeVector2D` _locationx _locationy))
  (bind (_x _y) (`KismetMathLibrary.BreakVector2D` (- (`self.TouchStart2DVector`) (`self.TouchEnd2DVector`))))
  ;[1 1 1] Touch Controls
  (`|ExecutionSequence`
    (:`then_1`
      (if (`self.IsPressed`)
        (if (> (`KismetMathLibrary.VSize2D` (- (`self.TouchStart2DVector`) _returnvalue)) 100.0)
          (`/Engine/EditorBlueprintResources/StandardMacros.DoOnce` false :!label _label
            (:`Completed`
              (set `self.TouchEnd2DVector` _returnvalue)
              (if (> (`KismetMathLibrary.Abs` _x) (`KismetMathLibrary.Abs` _y))
                (if (> _x 0.0)
                  (`KismetSystemLibrary.PrintString` "Left")
                  ;[1 1 1] Left/Right Movement & Jump
                  (set `self.NewLane` (`KismetMathLibrary.Clamp` (+ (`self.Lane`) -1) 0 2) :!label _label_2)
                  (bind (_direction _laney_2) (`Timeline|Lerp Timeline` :!via `PlayFromStart` :!label _label_3)
                    (:`Update`
                      (`self.K2_SetActorLocation` (`KismetMathLibrary.MakeVector` _returnvalue_x (`KismetMathLibrary.Lerp` (`|GetArrayItem` _laney (`self.Lane`)) (`|GetArrayItem` _laney (`self.NewLane`)) _laney_2) _returnvalue_z)))
                    (:`Finished`
                      (set `self.Lane` (`self.NewLane`))))
                  (else
                    (`KismetSystemLibrary.PrintString` "Right")
                    (set `self.NewLane` (`KismetMathLibrary.Clamp` (+ (`self.Lane`) 1) 0 2) :!label _label_4)
                    (goto _label_3 :!via `PlayFromStart`)))
                (elif (> _y 0.0)
                  (`KismetSystemLibrary.PrintString` "Up")
                  (`self.Jump` :!label _label_5)
                  (`GameplayStatics.PlaySound2D` "/Game/SFX/SFX_Jump.SFX_Jump" 1.0 1.0 0.0 null null)
                  (else
                    (`KismetSystemLibrary.PrintString` "Down")
                    (`CharacterMovementComponent.AddImpulse` (`self.CharacterMovement`) (0.0 0.0 -3000.0) true :!label _label_6)))))))))))

(event `Key|Left`
  (params (Key :type "Key Structure"))
  ;[1 1 1] Left/Right Movement & Jump
  (:`Pressed`
    (goto _label_2)))

(event `InputAction|Finger 1`
  (params (Key :type "Key Structure"))
  (bind (_locationx _locationy) (`PlayerController.GetInputTouchState` (`GameplayStatics.GetPlayerController` 0) "Touch1"))
  ;[1 1 1] Touch Controls
  (:`Pressed`
    (set `self.IsPressed` true)
    (set `self.TouchStart2DVector` (`KismetMathLibrary.MakeVector2D` _locationx _locationy)))
  (:`Released`
    (set `self.IsPressed` false)
    (goto _label :!via `Reset`)))

(event `Key|Right`
  (params (Key :type "Key Structure"))
  ;[1 1 1] Left/Right Movement & Jump
  (:`Pressed`
    (goto _label_4)))

(event `InputAction|Jump`
  (params (Key :type "Key Structure"))
  ;[1 1 1] Left/Right Movement & Jump
  (:`Pressed`
    (goto _label_5))
  (:`Released`
    (`self.StopJumping`)))

(event `InputAction|Lower`
  (params (Key :type "Key Structure"))
  (:`Pressed`
    (goto _label_6)))

(fn `DeathFunction`
  (`PrimitiveComponent.SetSimulatePhysics` (`self.Mesh`) true)
  (`CharacterMovementComponent.DisableMovement` (`self.CharacterMovement`))
  (bind _returnvalue (`|CreateWidget` "/Game/UI/WPB_GameOver.WPB_GameOver_C"))
  (`UserWidget.AddToViewport` _returnvalue 0)
  (bind _asbp_adrenaline_alley_game_mode (cast `/Game/Blueprints/GameModes/BP_AdrenalineAlleyGameMode` (`GameplayStatics.GetGameMode`)))
  (bind _returnvalue_2 (`GameplayStatics.DoesSaveGameExist` "HighscoreData"))
  (if _returnvalue_2
    (bind _returnvalue_3 (`GameplayStatics.LoadGameFromSlot` "HighscoreData"))
    (bind _output_get (set `self.SaverSubClass` _returnvalue_3))
    (bind _asbp_save_game (cast `/Game/Blueprints/SaveGames/BP_SaveGame` _output_get))
    (bind _currentpoints (`/Game/Blueprints/GameModes/BP_AdrenalineAlleyGameMode.CurrentPoints` _asbp_adrenaline_alley_game_mode))
    (if (> _currentpoints (`/Game/Blueprints/SaveGames/BP_SaveGame.HighscoreValue` _asbp_save_game))
      (set `/Game/Blueprints/SaveGames/BP_SaveGame.HighscoreValue` _currentpoints _asbp_save_game)
      (`GameplayStatics.SaveGameToSlot` (`self.SaverSubClass`) "HighscoreData"))
    (else
      (bind _returnvalue_4 (`GameplayStatics.CreateSaveGameObject` "/Game/Blueprints/SaveGames/BP_SaveGame.BP_SaveGame_C"))
      (bind _output_get_2 (set `self.SaverSubClass` _returnvalue_4))
      (bind _asbp_save_game_2 (cast `/Game/Blueprints/SaveGames/BP_SaveGame` _output_get_2))
      (set `/Game/Blueprints/SaveGames/BP_SaveGame.HighscoreValue` _currentpoints _asbp_save_game_2)
      (`GameplayStatics.SaveGameToSlot` (`self.SaverSubClass`) "HighscoreData"))))

(fn `UserConstructionScript`)