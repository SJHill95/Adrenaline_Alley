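; Item spawner Blueprint that periodically drops items at its own location while the level is being played.
; On BeginPlay it finds the level manager, then loops through a random delay between min and max, spawning via the parent's SpawnItem and moving the item to the spawner.
; The loop re-arms only while the level manager reports playing.
; Spawned actors that hit the out-of-bounds limit are destroyed after the parent handler runs.
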(event `self.ReceiveBeginPlay`
  (bind (_levelmanager _levelmanagerfound) (`/Game/Blueprints/Libraries/BPF_Lib.GetLevelManager`))
  (if _levelmanagerfound
    (set `self.LevelManagerRef` _levelmanager)
    (`self.LineUpNextItemSpawn`)))

(event `LineUpNextItemSpawn`
  (`KismetSystemLibrary.Delay` (`KismetMathLibrary.RandomFloatInRange` (`self.MinDelay`) (`self.MaxDelay`)))
  (`self.PlaceItem`)
  (if (`/Game/Blueprints/Game/BP_LevelManager.bIsPlaying` (`self.LevelManagerRef`))
    (`self.LineUpNextItemSpawn`)))

(fn `PlaceItem`
  (bind _returnvalue (`self.SpawnItem`))
  (`self.K2_SetActorLocation` _returnvalue (`self.K2_GetActorLocation`) false false))

(fn `SpawnActor`
  (returns (ReturnValue :type "Actor Object Reference"))
  (bind _returnvalue (`parent.SpawnActor`))
  (return _returnvalue))

(fn `SpawnedActorHitBounds`
  (params (OutOfBoundsActor :type "Actor Object Reference"))
  (`parent.SpawnedActorHitBounds` null)
  (`self.K2_DestroyActor` OutOfBoundsActor))

(fn `SpawnItem`
  (returns (ReturnValue :type "Actor Object Reference"))
  (bind _returnvalue (`parent.SpawnItem`))
  (return _returnvalue))

(fn `UserConstructionScript`
  (`parent.UserConstructionScript`))