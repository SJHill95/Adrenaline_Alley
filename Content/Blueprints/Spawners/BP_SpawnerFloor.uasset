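; Floor spawner Blueprint that lays out a row of tiles along X and recycles them to keep the floor continuous.
; On BeginPlay it spawns the required count through the parent's SpawnActor, placing the first at the spawner and chaining the rest behind RearTile.
; Tile spacing comes from the first tile's X bounds, slightly under full width.
; When a tile hits bounds, it moves behind RearTile and becomes the new RearTile.
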(event `self.ReceiveBeginPlay`
  (bind (_returnvalue_x _returnvalue_y) (`KismetMathLibrary.BreakVector` (`self.K2_GetActorLocation` (`self.RearTile`))))
  (`parent.ReceiveBeginPlay`)
  (for _index (range (+ (`self.ActorRequiredCount`) 1))
    (if (== _index 0)
      (bind _returnvalue (`self.SpawnActor`))
      (set `self.RearTile` _returnvalue)
      (set `self.TileSize` (* (.x (`.BoxExtent` (`self.GetActorBounds` _returnvalue false false))) 1.9))
      (`self.K2_SetActorLocation` (`self.RearTile`) (`self.K2_GetActorLocation`) false false)
      (else
        (bind _returnvalue_2 (`self.SpawnActor`))
        (`self.K2_SetActorLocation` _returnvalue_2 (`KismetMathLibrary.MakeVector` (+ _returnvalue_x (`self.TileSize`)) _returnvalue_y) false false)
        (set `self.RearTile` _returnvalue_2)))))

(fn `SpawnActor`
  (returns (ReturnValue :type "Actor Object Reference"))
  (bind _returnvalue (`parent.SpawnActor`))
  (return _returnvalue))

(fn `SpawnedActorHitBounds`
  (params (OutOfBoundsActor :type "Actor Object Reference"))
  (bind (_returnvalue_x _returnvalue_y _returnvalue_z) (`KismetMathLibrary.BreakVector` (`self.K2_GetActorLocation` (`self.RearTile`))))
  (`parent.SpawnedActorHitBounds` null)
  (`self.K2_SetActorLocation` OutOfBoundsActor (`KismetMathLibrary.MakeVector` (+ _returnvalue_x (`self.TileSize`)) _returnvalue_y _returnvalue_z) false false)
  (set `self.RearTile` OutOfBoundsActor))

(fn `UserConstructionScript`
  (`parent.UserConstructionScript`))