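; BP_Obstacle is an obstacle with randomized height that ends the game when the player character hits it.
; On mesh overlap, an active ghost state disables the mesh's collision; otherwise it notifies the player, then, if a level manager is found, plays an impact sound and triggers game over.
; The construction script randomizes vertical scale, and simple accessors store and return a parent reference.
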(event `self.StaticMesh.OnComponentBeginOverlap`
  (params (OverlappedComponent :type "PrimitiveComponent Object Reference") (OtherActor :type "Actor Object Reference") (OtherComp :type "PrimitiveComponent Object Reference") (OtherBodyIndex :type Integer) (bFromSweep :type Boolean) (SweepResult :type "HitResult Structure (by ref)"))
  (bind (_levelmanager _levelmanagerfound) (`/Game/Blueprints/Libraries/BPF_Lib.GetLevelManager`))
  (bind _asbp_player_character (cast `/Game/Blueprints/Characters/BP_PlayerCharacter` OtherActor))
  (if (`/Game/Blueprints/Characters/BP_PlayerCharacter.GhostActive` _asbp_player_character)
    (`PrimitiveComponent.SetCollisionEnabled` (`self.StaticMesh`) "NoCollision")
    (else
      (`/Game/Blueprints/Characters/BP_PlayerCharacter.HitObstacle` _asbp_player_character)
      (if _levelmanagerfound
        (`GameplayStatics.PlaySound2D` "/Game/SFX/SFX_Impact.SFX_Impact" 1.0 1.0 0.0 null null)
        (`/Game/Blueprints/Game/BP_LevelManager.GameOver` _levelmanager)))))

(fn `ReturnParent`
  (returns (Parent :type "/Game/Blueprints/Spawners/BP_SpawnerBase Object Reference"))
  (return (`self.ParentRef`)))

(fn `SetParent`
  (params (Parent :type "/Game/Blueprints/Spawners/BP_SpawnerBase Object Reference"))
  (returns (Return :type Boolean))
  (set `self.ParentRef` Parent)
  (return false))

(fn `UserConstructionScript`
  (`SceneComponent.SetWorldScale3D` (`self.StaticMesh`) (`KismetMathLibrary.MakeVector` 1.0 2.0 (`KismetMathLibrary.RandomFloatInRange` 2.0 5.0))))