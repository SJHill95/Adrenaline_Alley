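; Player character for a lane-based runner with swipe and key controls, apparently a backup copy, that creates the HUD and reads lane setup from the level manager.
; Tick turns touch drags into one swipe per press, sharing logic with key inputs for timeline-eased lane changes, jumping and a downward slam impulse.
; Hitting an obstacle ragdolls the mesh, shows the game-over widget and saves the game mode's points if they beat the stored highscore.
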(event `Key|Tab` :paused true
  (params (Key :type "Key Structure"))
  (:`Pressed`
    (`GameplayStatics.SetGamePaused` true)))

(event `self.ReceiveBeginPlay`
  (bind _returnvalue (`|CreateWidget` "/Game/UI/HUD/WBP_HUD.WBP_HUD_C"))
  (bind _output_get (set `self.HUD` _returnvalue))
  (`UserWidget.AddToViewport` _output_get 0)
  (`self.Initialise`))

(event `self.ReceiveTick`
  (params (DeltaSeconds :type "Float (single-precision)"))
  (bind (_returnvalue_x _returnvalue_y) (`KismetMathLibrary.BreakVector` (`self.K2_GetActorLocation`)))
  (bind (_returnvalue_x_2 _returnvalue_y_2 _returnvalue_z) (`KismetMathLibrary.BreakVector` (`self.K2_GetActorLocation`)))
  (bind (_returnvalue_x_3 _returnvalue_y_3) (`KismetMathLibrary.BreakVector` (`self.K2_GetActorLocation`)))
  (bind (_returnvalue_x_4 _returnvalue_y_4 _returnvalue_z_2) (`KismetMathLibrary.BreakVector` (`self.K2_GetActorLocation`)))
  (bind (_locationx _locationy) (`PlayerController.GetInputTouchState` (`GameplayStatics.GetPlayerController` 0) "Touch1"))
  (bind _returnvalue (`KismetMathLibrary.MakeVector2D` _locationx _locationy))
  (bind (_x _y) (`KismetMathLibrary.BreakVector2D` (- (`self.TouchStart2DVector`) (`self.TouchEnd2DVector`))))
  ;[1 1 1] Touch Controls
  (`|ExecutionSequence`
    (:`then_1`
      (if (`self.IsPressed`)
        (if (> (`KismetMathLibrary.VSize2D` (- (`self.TouchStart2DVector`) _returnvalue)) 100.0)
          (`/Engine/EditorBlueprintResources/StandardMacros.DoOnce` false :!label _label
            (:`Completed`
              (set `self.TouchEnd2DVector` _returnvalue)
              (if (> (`KismetMathLibrary.Abs` _x) (`KismetMathLibrary.Abs` _y))
                (if (> _x 0.0)
                  ;[1 1 1] Left/Right Movement & Jump
                  (if (`/Game/Blueprints/Game/BP_LevelManager.bIsPlaying` (`self.LevelManagerRef`)) :!label _label_2
                    (if (<= (`self.CurrentLane`) 1)
                      _
                      (elif (not (`self.bMoving`))
                        (set `self.bMoving` true)
                        (set `self.TargetPosition` (- _returnvalue_y_3 (`self.LaneWidth`)))
                        (bind (_direction _move) (`Timeline|MoveLeft` :!via `PlayFromStart`)
                          (:`Update`
                            (`self.K2_SetActorLocation` (`KismetMathLibrary.MakeVector` _returnvalue_x_4 (`KismetMathLibrary.Lerp` _returnvalue_y_4 (`self.TargetPosition`) _move) _returnvalue_z_2)))
                          (:`Finished`
                            (set `self.bMoving` false)
                            (`/Engine/EditorBlueprintResources/StandardMacros.DecrementInt` (`self.CurrentLane`)))))))
                  (else
                    (if (`/Game/Blueprints/Game/BP_LevelManager.bIsPlaying` (`self.LevelManagerRef`)) :!label _label_3
                      (if (== (`self.CurrentLane`) (`/Game/Blueprints/Game/BP_LevelManager.NumberOfLanes` (`self.LevelManagerRef`)))
                        _
                        (elif (not (`self.bMoving`))
                          (set `self.bMoving` true)
                          (set `self.TargetPosition` (+ _returnvalue_y (`self.LaneWidth`)))
                          (bind (_direction_2 _move_2) (`Timeline|MoveRight` :!via `PlayFromStart`)
                            (:`Update`
                              (`self.K2_SetActorLocation` (`KismetMathLibrary.MakeVector` _returnvalue_x_2 (`KismetMathLibrary.Lerp` _returnvalue_y_2 (`self.TargetPosition`) _move_2) _returnvalue_z)))
                            (:`Finished`
                              (set `self.bMoving` false)
                              (`/Engine/EditorBlueprintResources/StandardMacros.IncrementInt` (`self.CurrentLane`)))))))))
                (elif (> _y 0.0)
                  (if (`/Game/Blueprints/Game/BP_LevelManager.bIsPlaying` (`self.LevelManagerRef`)) :!label _label_4
                    (`self.Jump`)
                    (`GameplayStatics.PlaySound2D` "/Game/SFX/soundtrack/SFX_Jump02.SFX_Jump02" 1.0 1.0 0.0 null null))
                  (else
                    (`CharacterMovementComponent.AddImpulse` (`self.CharacterMovement`) (0.0 0.0 -3000.0) true :!label _label_5)))))))))))

(event `Key|Left`
  (params (Key :type "Key Structure"))
  ;[1 1 1] Left/Right Movement & Jump
  (:`Pressed`
    (goto _label_2)))

(event `InputAction|Finger 1`
  (params (Key :type "Key Structure"))
  (bind (_locationx _locationy) (`PlayerController.GetInputTouchState` (`GameplayStatics.GetPlayerController` 0) "Touch1"))
  ;[1 1 1] Touch Controls
  (:`Pressed`
    (set `self.IsPressed` true)
    (set `self.TouchStart2DVector` (`KismetMathLibrary.MakeVector2D` _locationx _locationy)))
  (:`Released`
    (set `self.IsPressed` false)
    (goto _label :!via `Reset`)))

(event `Key|Right`
  (params (Key :type "Key Structure"))
  ;[1 1 1] Left/Right Movement & Jump
  (:`Pressed`
    (goto _label_3)))

(event `InputAction|Jump`
  (params (Key :type "Key Structure"))
  ;[1 1 1] Left/Right Movement & Jump
  (:`Pressed`
    (goto _label_4))
  (:`Released`
    (`self.StopJumping`)
    (`KismetSystemLibrary.Delay` 0.8)
    (`GameplayStatics.PlaySound2D` "/Game/SFX/soundtrack/Jump_part_2.Jump_part_2" 1.0 1.0 0.0 null null)))

(event `InputAction|Lower`
  (params (Key :type "Key Structure"))
  (:`Pressed`
    (goto _label_5)))

(fn `DeathFunction`
  (`PrimitiveComponent.SetSimulatePhysics` (`self.Mesh`) true)
  (`WidgetLayoutLibrary.RemoveAllWidgets`)
  (bind _returnvalue (`|CreateWidget` "/Game/UI/GameOver/WPB_GameOver.WPB_GameOver_C"))
  (`UserWidget.AddToViewport` _returnvalue 0)
  (bind _asbp_adrenaline_alley_game_mode (cast `/Game/Blueprints/GameModes/BP_AdrenalineAlleyGameMode` (`GameplayStatics.GetGameMode`)))
  (bind _returnvalue_2 (`GameplayStatics.DoesSaveGameExist` "HighscoreData"))
  (if _returnvalue_2
    (bind _returnvalue_3 (`GameplayStatics.LoadGameFromSlot` "HighscoreData"))
    (bind _output_get (set `self.SaverSubClass` _returnvalue_3))
    (bind _asbp_save_game (cast `/Game/Blueprints/SaveGames/BP_SaveGame` _output_get))
    (bind _currentpoints (`/Game/Blueprints/GameModes/BP_AdrenalineAlleyGameMode.CurrentPoints` _asbp_adrenaline_alley_game_mode))
    (if (> _currentpoints (`/Game/Blueprints/SaveGames/BP_SaveGame.HighscoreValue` _asbp_save_game))
      (set `/Game/Blueprints/SaveGames/BP_SaveGame.HighscoreValue` _currentpoints _asbp_save_game)
      (`GameplayStatics.SaveGameToSlot` (`self.SaverSubClass`) "HighscoreData"))
    (else
      (bind _returnvalue_4 (`GameplayStatics.CreateSaveGameObject` "/Game/Blueprints/SaveGames/BP_SaveGame.BP_SaveGame_C"))
      (bind _output_get_2 (set `self.SaverSubClass` _returnvalue_4))
      (bind _asbp_save_game_2 (cast `/Game/Blueprints/SaveGames/BP_SaveGame` _output_get_2))
      (set `/Game/Blueprints/SaveGames/BP_SaveGame.HighscoreValue` _currentpoints _asbp_save_game_2)
      (`GameplayStatics.SaveGameToSlot` (`self.SaverSubClass`) "HighscoreData"))))

(fn `HitObstacle`
  (`GameplayStatics.PlaySound2D` "/Game/SFX/soundtrack/SFX_Crash.SFX_Crash" 1.0 1.0 0.0 null null)
  (`self.DeathFunction`))

(fn `Initialise`
  (bind (_levelmanager _levelmanagerfound) (`/Game/Blueprints/Libraries/BPF_Lib.GetLevelManager`))
  (if _levelmanagerfound
    (set `self.LevelManagerRef` _levelmanager)
    (set `self.CurrentLane` (+ (/ (`/Game/Blueprints/Game/BP_LevelManager.NumberOfLanes` (`self.LevelManagerRef`)) 2) 1))
    (set `self.LaneWidth` (`/Game/Blueprints/Game/BP_LevelManager.LaneWidth` (`self.LevelManagerRef`)))
    (else
      (`KismetSystemLibrary.PrintString` "No Level Manager found"))))

(fn `UserConstructionScript`)