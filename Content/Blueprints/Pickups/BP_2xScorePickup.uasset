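; BP_2xScorePickup is a spinning pickup that grants the player a temporary double-score state.
; BeginPlay sets the yaw spin rate.
; On player overlap, a branch on the active flag either resets a DoOnce or enters it to set the flag, play the HUD fadeout animation and hide the pickup.
; After a fixed delay, it clears the flag on player 0's character and destroys itself.
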(event `self.ReceiveBeginPlay`
  ;[1 1 1] Rotation
  (set `self.YawPerSecond` 200.0)
  (set `self.PitchPerSecond` 0.0))

(event `self.Pickup.OnComponentBeginOverlap`
  (params (OverlappedComponent :type "PrimitiveComponent Object Reference") (OtherActor :type "Actor Object Reference") (OtherComp :type "PrimitiveComponent Object Reference") (OtherBodyIndex :type Integer) (bFromSweep :type Boolean) (SweepResult :type "HitResult Structure (by ref)"))
  ;[1 1 1] Sets 2x Score active
  (bind _asbp_player_character (cast `/Game/Blueprints/Characters/BP_PlayerCharacter` OtherActor))
  (if (`/Game/Blueprints/Characters/BP_PlayerCharacter.2xScoreActive` _asbp_player_character)
    (goto _label :!via `Reset`)
    (else
      (`/Engine/EditorBlueprintResources/StandardMacros.DoOnce` false :!label _label
        (:`Completed`
          (set `/Game/Blueprints/Characters/BP_PlayerCharacter.2xScoreActive` true _asbp_player_character)
          (bind _hud (`/Game/Blueprints/Characters/BP_PlayerCharacter.HUD` _asbp_player_character))
          (`UserWidget.PlayAnimation` _hud (`/Game/UI/HUD/WBP_HUD.2xScoreFadeout` _hud) 0.0 1 "Forward" 1.0 false)
          (`SceneComponent.SetVisibility` (`self.Pickup`) false true)
          (`KismetSystemLibrary.Delay` 10.0)
          (bind _asbp_player_character_2 (cast `/Game/Blueprints/Characters/BP_PlayerCharacter` (`GameplayStatics.GetPlayerCharacter` 0)))
          (set `/Game/Blueprints/Characters/BP_PlayerCharacter.2xScoreActive` false _asbp_player_character_2)
          (`self.K2_DestroyActor`))))))

(fn `UserConstructionScript`
  (`parent.UserConstructionScript`))