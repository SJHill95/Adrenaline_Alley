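; Starter track tile for an endless runner with three obstacle lanes.
; When the player overlaps its Box, it has the game mode spawn the next tile, adds multiplied points, raises walk speed slightly within a clamp, then destroys itself after a short delay.
; SpawnObstacles randomly places obstacles or coins per lane, rolling each next lane only if the previous one spawned; nothing in this Blueprint calls it.
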(event `self.Box.OnComponentBeginOverlap`
  (params (OverlappedComponent :type "PrimitiveComponent Object Reference") (OtherActor :type "Actor Object Reference") (OtherComp :type "PrimitiveComponent Object Reference") (OtherBodyIndex :type Integer) (bFromSweep :type Boolean) (SweepResult :type "HitResult Structure (by ref)"))
  (cast `/Game/Blueprints/Characters/BP_PlayerCharacter` OtherActor)
  (bind _asbp_adrenaline_alley_game_mode (cast `/Game/Blueprints/GameModes/BP_AdrenalineAlleyGameMode` (`GameplayStatics.GetGameMode`)))
  (`/Game/Blueprints/GameModes/BP_AdrenalineAlleyGameMode.SpawnTile` _asbp_adrenaline_alley_game_mode)
  (bind _asbp_adrenaline_alley_game_mode_2 (cast `/Game/Blueprints/GameModes/BP_AdrenalineAlleyGameMode` (`GameplayStatics.GetGameMode`)))
  (set `/Game/Blueprints/GameModes/BP_AdrenalineAlleyGameMode.CurrentPoints` (+ (* 1 (`/Game/Blueprints/GameModes/BP_AdrenalineAlleyGameMode.PointsMultiplier` _asbp_adrenaline_alley_game_mode_2)) (`/Game/Blueprints/GameModes/BP_AdrenalineAlleyGameMode.CurrentPoints` _asbp_adrenaline_alley_game_mode_2)) _asbp_adrenaline_alley_game_mode_2)
  (bind _asbp_player_character (cast `/Game/Blueprints/Characters/BP_PlayerCharacter` (`GameplayStatics.GetPlayerCharacter` 0)))
  (bind _charactermovement (`Character.CharacterMovement` _asbp_player_character))
  (set `CharacterMovementComponent.MaxWalkSpeed` (`KismetMathLibrary.FClamp` (* (`CharacterMovementComponent.MaxWalkSpeed` _charactermovement) 1.01) 1000.0 2000.0) _charactermovement)
  (`KismetSystemLibrary.Delay` 0.5)
  (`self.K2_DestroyActor`))

(event `self.ReceiveBeginPlay`)

(fn `SpawnObstacles`
  (bind _returnvalue (`SceneComponent.K2_GetComponentToWorld` (`self.Lane2`)))
  (bind _returnvalue_2 (`SceneComponent.K2_GetComponentToWorld` (`self.Lane1`)))
  (bind _returnvalue_3 (`SceneComponent.K2_GetComponentToWorld` (`self.Lane0`)))
  ;[1 1 1] Lane 0
  (switch `int` (`KismetMathLibrary.RandomIntegerInRange` 0 12)
    (:`1`
      (`|SpawnActorFromClass` "/Game/Blueprints/Obstacles/BP_Obstacle01.BP_Obstacle01_C" _returnvalue_3 "Undefined" "OverrideRootScale" null null))
    (:`2`
      (`|SpawnActorFromClass` "/Game/Blueprints/Obstacles/BP_Obstacle02.BP_Obstacle02_C" _returnvalue_3 "Undefined" "OverrideRootScale" null null))
    (:`3`
      (`|SpawnActorFromClass` "/Game/Blueprints/Pickups/BP_CoinPickup.BP_CoinPickup_C" _returnvalue_3 "Undefined" "OverrideRootScale" null null)))
  ;[1 1 1] Lane 1
  (switch `int` (`KismetMathLibrary.RandomIntegerInRange` 0 6)
    (:`1`
      (`|SpawnActorFromClass` "/Game/Blueprints/Obstacles/BP_Obstacle01.BP_Obstacle01_C" _returnvalue_2 "Undefined" "OverrideRootScale" null null))
    (:`2`
      (`|SpawnActorFromClass` "/Game/Blueprints/Obstacles/BP_Obstacle02.BP_Obstacle02_C" _returnvalue_2 "Undefined" "OverrideRootScale" null null))
    (:`3`
      (`|SpawnActorFromClass` "/Game/Blueprints/Pickups/BP_CoinPickup.BP_CoinPickup_C" _returnvalue_2 "Undefined" "OverrideRootScale" null null)))
  ;[1 1 1] Lane 2
  (switch `int` (`KismetMathLibrary.RandomIntegerInRange` 0 6)
    (:`1`
      (`|SpawnActorFromClass` "/Game/Blueprints/Obstacles/BP_Obstacle01.BP_Obstacle01_C" _returnvalue "Undefined" "OverrideRootScale" null null))
    (:`2`
      (`|SpawnActorFromClass` "/Game/Blueprints/Obstacles/BP_Obstacle02.BP_Obstacle02_C" _returnvalue "Undefined" "OverrideRootScale" null null))
    (:`3`
      (`|SpawnActorFromClass` "/Game/Blueprints/Pickups/BP_CoinPickup.BP_CoinPickup_C" _returnvalue "Undefined" "OverrideRootScale" null null))))

(fn `UserConstructionScript`)