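; BP_Magnet_ is a magnet power-up pickup that temporarily turns on the player character's MagnetActive flag.
; Overlap feeds a DoOnce, entered if the magnet is inactive and reset otherwise, which sets the flag, plays a sound and starts the HUD's MagnetFadeOut animation.
; The pickup component is hidden and moved away while the actor waits out PickupTimer, then clears the flag and destroys itself.
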(event `self.Pickup.OnComponentBeginOverlap`
  (params (OverlappedComponent :type "PrimitiveComponent Object Reference") (OtherActor :type "Actor Object Reference") (OtherComp :type "PrimitiveComponent Object Reference") (OtherBodyIndex :type Integer) (bFromSweep :type Boolean) (SweepResult :type "HitResult Structure (by ref)"))
  ;[1 1 1] Magnet Pickup
  (bind _asbp_player_character (cast `/Game/Characters/BP_PlayerCharacter` OtherActor))
  (if (`/Game/Characters/BP_PlayerCharacter.MagnetActive` _asbp_player_character)
    (goto _label :!via `Reset`)
    (else
      (`/Engine/EditorBlueprintResources/StandardMacros.DoOnce` false :!label _label
        (:`Completed`
          (set `/Game/Characters/BP_PlayerCharacter.MagnetActive` true _asbp_player_character)
          (`SceneComponent.K2_SetWorldLocation` (`self.Pickup`) (0.0 0.0 5000.0) false false)
          (`SceneComponent.SetVisibility` (`self.Pickup`) false false)
          (`GameplayStatics.PlaySound2D` "/Game/Sounds/SFX/S_Magnet_Cue.S_Magnet_Cue" 1.0 1.0 0.0 null null)
          (bind _hud (`/Game/Characters/BP_PlayerCharacter.HUD` _asbp_player_character))
          (`UserWidget.PlayAnimation` _hud (`/Game/UI/HUD/WBP_HUD.MagnetFadeOut` _hud) 0.0 1 "Forward" 1.0 false)
          (`KismetSystemLibrary.Delay` (`self.PickupTimer`))
          (bind _asbp_player_character_2 (cast `/Game/Characters/BP_PlayerCharacter` (`GameplayStatics.GetPlayerCharacter` 0)))
          (set `/Game/Characters/BP_PlayerCharacter.MagnetActive` false _asbp_player_character_2)
          (`self.K2_DestroyActor`))))))

(fn `Magnet`)

(fn `UserConstructionScript`
  (`parent.UserConstructionScript`))