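; Ramp obstacle actor that carries its own row of coins and clears out gold coins that overlap it.
; On BeginPlay, SpawnCoins creates five BP_RampCoin actors below the world origin, then teleport-free moves each to its spawn point component.
; Any BP_GoldCoin overlapping the ramp's static mesh is destroyed with a debug print.
; SetParent and ReturnParent store and expose a ParentRef.
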(event `self.ReceiveBeginPlay`
  (`self.SpawnCoins`))

(event `self.StaticMesh.OnComponentBeginOverlap`
  (params (OverlappedComponent :type "PrimitiveComponent Object Reference") (OtherActor :type "Actor Object Reference") (OtherComp :type "PrimitiveComponent Object Reference") (OtherBodyIndex :type Integer) (bFromSweep :type Boolean) (SweepResult :type "HitResult Structure (by ref)"))
  (bind _asbp_gold_coin (cast `/Game/Blueprints/Pickups/BP_GoldCoin` OtherActor))
  (`self.K2_DestroyActor` _asbp_gold_coin)
  (`KismetSystemLibrary.PrintString` "Coin Destroyed"))

(fn `ReturnParent`
  (returns (Parent :type "/Game/Blueprints/Spawners/BP_SpawnerBase Object Reference"))
  (return (`self.ParentRef`)))

(fn `SetParent`
  (params (Parent :type "/Game/Blueprints/Spawners/BP_SpawnerBase Object Reference"))
  (returns (Return :type Boolean))
  (set `self.ParentRef` Parent)
  (return false))

(fn `SpawnCoins`
  (`|ExecutionSequence`
    (:`then_0`
      (set `self.CoinLocation01` (`SceneComponent.K2_GetComponentLocation` (`self.CoinSpawnPoint01`)))
      (bind _returnvalue (`|SpawnActorFromClass` "/Game/Blueprints/Pickups/BP_RampCoin.BP_RampCoin_C" (`KismetMathLibrary.MakeTransform` (0.0 0.0 -1000.0)) "Undefined" "OverrideRootScale" null null))
      (`self.K2_SetActorLocation` _returnvalue (`self.CoinLocation01`) false false))
    (:`then_1`
      (set `self.CoinLocation02` (`SceneComponent.K2_GetComponentLocation` (`self.CoinSpawnPoint02`)))
      (bind _returnvalue_2 (`|SpawnActorFromClass` "/Game/Blueprints/Pickups/BP_RampCoin.BP_RampCoin_C" (`KismetMathLibrary.MakeTransform` (0.0 0.0 -1000.0)) "Undefined" "OverrideRootScale" null null))
      (`self.K2_SetActorLocation` _returnvalue_2 (`self.CoinLocation02`) false false))
    (:`then_2`
      (set `self.CoinLocation03` (`SceneComponent.K2_GetComponentLocation` (`self.CoinSpawnPoint03`)))
      (bind _returnvalue_3 (`|SpawnActorFromClass` "/Game/Blueprints/Pickups/BP_RampCoin.BP_RampCoin_C" (`KismetMathLibrary.MakeTransform` (0.0 0.0 -1000.0)) "Undefined" "OverrideRootScale" null null))
      (`self.K2_SetActorLocation` _returnvalue_3 (`self.CoinLocation03`) false false))
    (:`then_3`
      (set `self.CoinLocation04` (`SceneComponent.K2_GetComponentLocation` (`self.CoinSpawnPoint04`)))
      (bind _returnvalue_4 (`|SpawnActorFromClass` "/Game/Blueprints/Pickups/BP_RampCoin.BP_RampCoin_C" (`KismetMathLibrary.MakeTransform` (0.0 0.0 -1000.0)) "Undefined" "OverrideRootScale" null null))
      (`self.K2_SetActorLocation` _returnvalue_4 (`self.CoinLocation04`) false false))
    (:`then_4`
      (set `self.CoinLocation05` (`SceneComponent.K2_GetComponentLocation` (`self.CoinSpawnPoint05`)))
      (bind _returnvalue_5 (`|SpawnActorFromClass` "/Game/Blueprints/Pickups/BP_RampCoin.BP_RampCoin_C" (`KismetMathLibrary.MakeTransform` (0.0 0.0 -1000.0)) "Undefined" "OverrideRootScale" null null))
      (`self.K2_SetActorLocation` _returnvalue_5 (`self.CoinLocation05`) false false))))

(fn `UserConstructionScript`)