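; Ramp obstacle that spawns a coin line on a randomly chosen left or right side at BeginPlay.
; Wall, side and railing triggers report a hit and end the game through the level manager, unless the player's ghost mode is active, which disables mesh collision.
; A timeline rotates the player for the left rail grind and reverses on exit.
; The mesh destroys overlapping gold coins; the ramp jump logic is unconnected.
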(event `self.ReceiveBeginPlay`
  (bind _returnvalue (`KismetMathLibrary.RandomFloatInRange` 0.1 0.9))
  ;[1 1 1] Spawn Coins
  (if (`KismetMathLibrary.InRange_FloatFloat` _returnvalue 0.0 0.5)
    (`self.SpawnCoinsL`)
    (elif (`KismetMathLibrary.InRange_FloatFloat` _returnvalue 0.5)
      (`self.SpawnCoinsR`))))

(event `self.Wall02Trigger.OnComponentBeginOverlap`
  (params (OverlappedComponent :type "PrimitiveComponent Object Reference") (OtherActor :type "Actor Object Reference") (OtherComp :type "PrimitiveComponent Object Reference") (OtherBodyIndex :type Integer) (bFromSweep :type Boolean) (SweepResult :type "HitResult Structure (by ref)"))
  (bind (_levelmanager _levelmanagerfound) (`/Game/Blueprints/Libraries/BPF_Lib.GetLevelManager`))
  ;[1 1 1] Wall02Trigger
  (bind _asbp_player_character (cast `/Game/Blueprints/Characters/BP_PlayerCharacter` OtherActor))
  (if (`/Game/Blueprints/Characters/BP_PlayerCharacter.GhostActive` _asbp_player_character)
    (`PrimitiveComponent.SetCollisionEnabled` (`self.StaticMesh`) "NoCollision")
    (else
      (`/Game/Blueprints/Characters/BP_PlayerCharacter.HitObstacle` _asbp_player_character)
      (if _levelmanagerfound
        (`/Game/Blueprints/Game/BP_LevelManager.GameOver` _levelmanager)))))

(event `self.Wall01Trigger.OnComponentBeginOverlap`
  (params (OverlappedComponent :type "PrimitiveComponent Object Reference") (OtherActor :type "Actor Object Reference") (OtherComp :type "PrimitiveComponent Object Reference") (OtherBodyIndex :type Integer) (bFromSweep :type Boolean) (SweepResult :type "HitResult Structure (by ref)"))
  (bind (_levelmanager _levelmanagerfound) (`/Game/Blueprints/Libraries/BPF_Lib.GetLevelManager`))
  ;[1 1 1] Wall01Trigger
  (bind _asbp_player_character (cast `/Game/Blueprints/Characters/BP_PlayerCharacter` OtherActor))
  (if (`/Game/Blueprints/Characters/BP_PlayerCharacter.GhostActive` _asbp_player_character)
    (`PrimitiveComponent.SetCollisionEnabled` (`self.StaticMesh`) "NoCollision")
    (else
      (`/Game/Blueprints/Characters/BP_PlayerCharacter.HitObstacle` _asbp_player_character)
      (if _levelmanagerfound
        (`/Game/Blueprints/Game/BP_LevelManager.GameOver` _levelmanager)))))

(event `self.StaticMesh.OnComponentBeginOverlap`
  (params (OverlappedComponent :type "PrimitiveComponent Object Reference") (OtherActor :type "Actor Object Reference") (OtherComp :type "PrimitiveComponent Object Reference") (OtherBodyIndex :type Integer) (bFromSweep :type Boolean) (SweepResult :type "HitResult Structure (by ref)"))
  ;[1 1 1] Destroys coins that spawn in obstacle
  (bind _asbp_gold_coin (cast `/Game/Blueprints/Pickups/BP_GoldCoin` OtherActor))
  (`self.K2_DestroyActor` _asbp_gold_coin)
  (`KismetSystemLibrary.PrintString` "Coin Destroyed"))

(event `self.RightRailingTrigger.OnComponentBeginOverlap`
  (params (OverlappedComponent :type "PrimitiveComponent Object Reference") (OtherActor :type "Actor Object Reference") (OtherComp :type "PrimitiveComponent Object Reference") (OtherBodyIndex :type Integer) (bFromSweep :type Boolean) (SweepResult :type "HitResult Structure (by ref)"))
  (bind (_levelmanager _levelmanagerfound) (`/Game/Blueprints/Libraries/BPF_Lib.GetLevelManager`))
  ;[1 1 1] RightRailingTrigger
  (bind _asbp_player_character (cast `/Game/Blueprints/Characters/BP_PlayerCharacter` OtherActor))
  (if (`/Game/Blueprints/Characters/BP_PlayerCharacter.GhostActive` _asbp_player_character)
    (`PrimitiveComponent.SetCollisionEnabled` (`self.StaticMesh`) "NoCollision")
    (else
      (`/Game/Blueprints/Characters/BP_PlayerCharacter.HitObstacle` _asbp_player_character)
      (if _levelmanagerfound
        (`/Game/Blueprints/Game/BP_LevelManager.GameOver` _levelmanager)))))

(event `self.FirstTrigger.OnComponentBeginOverlap`
  (params (OverlappedComponent :type "PrimitiveComponent Object Reference") (OtherActor :type "Actor Object Reference") (OtherComp :type "PrimitiveComponent Object Reference") (OtherBodyIndex :type Integer) (bFromSweep :type Boolean) (SweepResult :type "HitResult Structure (by ref)"))
  ;[1 1 1] Left Rail Grind
  (bind (_direction _rotate) (`Timeline|Timeline_0` :!via `PlayFromStart` :!label _label)
    (:`Update`
      (bind _asbp_player_character (cast `/Game/Blueprints/Characters/BP_PlayerCharacter` OtherActor))
      (`self.K2_SetActorRotation` _asbp_player_character (`KismetMathLibrary.RLerp` (`self.K2_GetActorRotation` _asbp_player_character) (struct :`Pitch` 20.0) _rotate) false))))

(event `self.LeftTrigger.OnComponentBeginOverlap`
  (params (OverlappedComponent :type "PrimitiveComponent Object Reference") (OtherActor :type "Actor Object Reference") (OtherComp :type "PrimitiveComponent Object Reference") (OtherBodyIndex :type Integer) (bFromSweep :type Boolean) (SweepResult :type "HitResult Structure (by ref)"))
  (bind (_levelmanager _levelmanagerfound) (`/Game/Blueprints/Libraries/BPF_Lib.GetLevelManager`))
  ;[1 1 1] LeftTrigger
  (bind _asbp_player_character (cast `/Game/Blueprints/Characters/BP_PlayerCharacter` OtherActor))
  (if (`/Game/Blueprints/Characters/BP_PlayerCharacter.GhostActive` _asbp_player_character)
    (`PrimitiveComponent.SetCollisionEnabled` (`self.StaticMesh`) "NoCollision")
    (else
      (`/Game/Blueprints/Characters/BP_PlayerCharacter.HitObstacle` _asbp_player_character)
      (if _levelmanagerfound
        (`/Game/Blueprints/Game/BP_LevelManager.GameOver` _levelmanager)))))

(event `self.FirstTrigger.OnComponentEndOverlap`
  (params (OverlappedComponent :type "PrimitiveComponent Object Reference") (OtherActor :type "Actor Object Reference") (OtherComp :type "PrimitiveComponent Object Reference") (OtherBodyIndex :type Integer))
  ;[1 1 1] Left Rail Grind
  (cast `/Game/Blueprints/Characters/BP_PlayerCharacter` OtherActor)
  (goto _label :!via `Reverse`))

(fn `ReturnParent`
  (returns (Parent :type "/Game/Blueprints/Spawners/BP_SpawnerBase Object Reference"))
  (return (`self.ParentRef`)))

(fn `SetParent`
  (params (Parent :type "/Game/Blueprints/Spawners/BP_SpawnerBase Object Reference"))
  (returns (Return :type Boolean))
  (set `self.ParentRef` Parent)
  (return false))

(fn `SpawnCoinsL`
  (`|ExecutionSequence`
    (:`then_0`
      (set `self.CoinLocation01` (`SceneComponent.K2_GetComponentLocation` (`self.CoinSpawnPoint01_L`)))
      (bind _returnvalue (`|SpawnActorFromClass` "/Game/Blueprints/Pickups/BP_RampCoin.BP_RampCoin_C" (`KismetMathLibrary.MakeTransform` (0.0 0.0 -1000.0)) "Undefined" "OverrideRootScale" null null))
      (`self.K2_SetActorLocation` _returnvalue (`self.CoinLocation01`) false false))
    (:`then_1`
      (set `self.CoinLocation02` (`SceneComponent.K2_GetComponentLocation` (`self.CoinSpawnPoint02_L`)))
      (bind _returnvalue_2 (`|SpawnActorFromClass` "/Game/Blueprints/Pickups/BP_RampCoin.BP_RampCoin_C" (`KismetMathLibrary.MakeTransform` (0.0 0.0 -1000.0)) "Undefined" "OverrideRootScale" null null))
      (`self.K2_SetActorLocation` _returnvalue_2 (`self.CoinLocation02`) false false))
    (:`then_2`
      (set `self.CoinLocation03` (`SceneComponent.K2_GetComponentLocation` (`self.CoinSpawnPoint03_L`)))
      (bind _returnvalue_3 (`|SpawnActorFromClass` "/Game/Blueprints/Pickups/BP_RampCoin.BP_RampCoin_C" (`KismetMathLibrary.MakeTransform` (0.0 0.0 -1000.0)) "Undefined" "OverrideRootScale" null null))
      (`self.K2_SetActorLocation` _returnvalue_3 (`self.CoinLocation03`) false false))
    (:`then_3`
      (set `self.CoinLocation04` (`SceneComponent.K2_GetComponentLocation` (`self.CoinSpawnPoint04_L`)))
      (bind _returnvalue_4 (`|SpawnActorFromClass` "/Game/Blueprints/Pickups/BP_RampCoin.BP_RampCoin_C" (`KismetMathLibrary.MakeTransform` (0.0 0.0 -1000.0)) "Undefined" "OverrideRootScale" null null))
      (`self.K2_SetActorLocation` _returnvalue_4 (`self.CoinLocation04`) false false))
    (:`then_4`
      (set `self.CoinLocation05` (`SceneComponent.K2_GetComponentLocation` (`self.CoinSpawnPoint05_L`)))
      (bind _returnvalue_5 (`|SpawnActorFromClass` "/Game/Blueprints/Pickups/BP_RampCoin.BP_RampCoin_C" (`KismetMathLibrary.MakeTransform` (0.0 0.0 -1000.0)) "Undefined" "OverrideRootScale" null null))
      (`self.K2_SetActorLocation` _returnvalue_5 (`self.CoinLocation05`) false false))))

(fn `SpawnCoinsR`
  (`|ExecutionSequence`
    (:`then_0`
      (set `self.CoinLocation01` (`SceneComponent.K2_GetComponentLocation` (`self.CoinSpawnPoint01_R`)))
      (bind _returnvalue (`|SpawnActorFromClass` "/Game/Blueprints/Pickups/BP_RampCoin.BP_RampCoin_C" (`KismetMathLibrary.MakeTransform` (0.0 0.0 -1000.0)) "Undefined" "OverrideRootScale" null null))
      (`self.K2_SetActorLocation` _returnvalue (`self.CoinLocation01`) false false))
    (:`then_1`
      (set `self.CoinLocation02` (`SceneComponent.K2_GetComponentLocation` (`self.CoinSpawnPoint02_R`)))
      (bind _returnvalue_2 (`|SpawnActorFromClass` "/Game/Blueprints/Pickups/BP_RampCoin.BP_RampCoin_C" (`KismetMathLibrary.MakeTransform` (0.0 0.0 -1000.0)) "Undefined" "OverrideRootScale" null null))
      (`self.K2_SetActorLocation` _returnvalue_2 (`self.CoinLocation02`) false false))
    (:`then_2`
      (set `self.CoinLocation03` (`SceneComponent.K2_GetComponentLocation` (`self.CoinSpawnPoint03_R`)))
      (bind _returnvalue_3 (`|SpawnActorFromClass` "/Game/Blueprints/Pickups/BP_RampCoin.BP_RampCoin_C" (`KismetMathLibrary.MakeTransform` (0.0 0.0 -1000.0)) "Undefined" "OverrideRootScale" null null))
      (`self.K2_SetActorLocation` _returnvalue_3 (`self.CoinLocation03`) false false))
    (:`then_3`
      (set `self.CoinLocation04` (`SceneComponent.K2_GetComponentLocation` (`self.CoinSpawnPoint04_R`)))
      (bind _returnvalue_4 (`|SpawnActorFromClass` "/Game/Blueprints/Pickups/BP_RampCoin.BP_RampCoin_C" (`KismetMathLibrary.MakeTransform` (0.0 0.0 -1000.0)) "Undefined" "OverrideRootScale" null null))
      (`self.K2_SetActorLocation` _returnvalue_4 (`self.CoinLocation04`) false false))
    (:`then_4`
      (set `self.CoinLocation05` (`SceneComponent.K2_GetComponentLocation` (`self.CoinSpawnPoint05_R`)))
      (bind _returnvalue_5 (`|SpawnActorFromClass` "/Game/Blueprints/Pickups/BP_RampCoin.BP_RampCoin_C" (`KismetMathLibrary.MakeTransform` (0.0 0.0 -1000.0)) "Undefined" "OverrideRootScale" null null))
      (`self.K2_SetActorLocation` _returnvalue_5 (`self.CoinLocation05`) false false))))

(fn `UserConstructionScript`)