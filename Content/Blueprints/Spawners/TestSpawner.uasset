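; Test spawner actor that randomly spawns a magnet or ghost item at its location on BeginPlay, then destroys itself after a SpawnRate delay.
; SpawnItems makes a fresh random roll for the second branch, so it yields roughly half magnets, a quarter ghosts and a quarter nothing.
; Tick only sets its interval to RespawnTime without respawning anything, and the coin spawn nodes are disconnected.
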(event `self.ReceiveTick`
  (params (DeltaSeconds :type "Float (single-precision)"))
  (`self.SetActorTickInterval` (`self.RespawnTime`)))

(event `self.ReceiveBeginPlay`
  (`self.SpawnItems`)
  (`KismetSystemLibrary.Delay` (`self.SpawnRate`))
  (`KismetSystemLibrary.PrintString` "Test Spawner Destroyed")
  (`self.K2_DestroyActor`))

(fn `SpawnItems`
  (bind _returnvalue (`KismetMathLibrary.RandomFloatInRange` 0.0 1.0))
  (if (`KismetMathLibrary.InRange_FloatFloat` _returnvalue 0.0 0.5)
    (`|SpawnActorFromClass` (`self.SpawnActor01`) (`KismetMathLibrary.MakeTransform` (`self.K2_GetActorLocation`)) "Undefined" "OverrideRootScale" null null)
    (`KismetSystemLibrary.PrintString` "Magnet spawned")
    (elif (`KismetMathLibrary.InRange_FloatFloat` _returnvalue 0.5)
      (`|SpawnActorFromClass` (`self.SpawnActor02`) (`KismetMathLibrary.MakeTransform` (`self.K2_GetActorLocation`)) "Undefined" "OverrideRootScale" null null)
      (`KismetSystemLibrary.PrintString` "Ghost spawned"))))

(fn `UserConstructionScript`)