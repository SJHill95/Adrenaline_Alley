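; Magnet pickup that turns on the player character's MagnetActive flag for a timed period when overlapped.
; A DoOnce gate triggers it if no magnet is active, while an overlap during an active magnet only resets the gate.
; Pickup moves away and hides, plays sound and HUD animations (shifting magnet UI if Ghost is active), then clears the flag and destroys itself after a delay.
; Getter and setter functions store a parent reference.
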(event `self.ReceiveActorBeginOverlap`
  (params (OtherActor :type "Actor Object Reference"))
  ;[1 1 1] Pickup
  (bind _asbp_player_character (cast `/Game/Blueprints/Characters/BP_PlayerCharacter` OtherActor))
  (if (`/Game/Blueprints/Characters/BP_PlayerCharacter.MagnetActive` _asbp_player_character)
    (goto _label :!via `Reset`)
    (else
      (`/Engine/EditorBlueprintResources/StandardMacros.DoOnce` false :!label _label
        (:`Completed`
          (set `/Game/Blueprints/Characters/BP_PlayerCharacter.MagnetActive` true _asbp_player_character)
          (`SceneComponent.K2_SetWorldLocation` (`self.Magnet`) (0.0 0.0 5000.0) false false)
          (`SceneComponent.SetVisibility` (`self.Magnet`) false false)
          (`GameplayStatics.PlaySound2D` "/Game/SFX/soundtrack/SFX_Magnet.SFX_Magnet" 1.0 1.0 0.0 null null)
          (if (`/Game/Blueprints/Characters/BP_PlayerCharacter.GhostActive` _asbp_player_character)
            (bind _hud (`/Game/Blueprints/Characters/BP_PlayerCharacter.HUD` _asbp_player_character))
            (`UserWidget.PlayAnimation` _hud (`/Game/UI/HUD/WBP_HUD.MoveMagnetUI` _hud) 0.0 1 "Forward" 1.0 true))
          (`UserWidget.PlayAnimation` _hud (`/Game/UI/HUD/WBP_HUD.ItemFadeOut` _hud) 0.0 1 "Forward" 1.0 false)
          (`KismetSystemLibrary.Delay` 10.0)
          (bind _asbp_player_character_2 (cast `/Game/Blueprints/Characters/BP_PlayerCharacter` (`GameplayStatics.GetPlayerCharacter` 0)))
          (set `/Game/Blueprints/Characters/BP_PlayerCharacter.MagnetActive` false _asbp_player_character_2)
          (`self.K2_DestroyActor`))))))

(fn `ReturnParent`
  (returns (Parent :type "/Game/Blueprints/Spawners/BP_SpawnerBase Object Reference"))
  (return (`self.ParentRef`)))

(fn `SetParent`
  (params (Parent :type "/Game/Blueprints/Spawners/BP_SpawnerBase Object Reference"))
  (returns (Return :type Boolean))
  (set `self.ParentRef` Parent)
  (return false))

(fn `UserConstructionScript`)