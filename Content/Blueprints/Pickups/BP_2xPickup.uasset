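; BP_2xPickup is a pickup that grants the player a temporary double-score state when overlapped.
; On overlap with BP_PlayerCharacter it sets the 2xScoreActive flag, plays the HUD's ItemFadeOut animation and hides its mesh.
; After a fixed delay it clears the flag on player character 0 and destroys itself; collision stays enabled during the wait.
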(event `self.ReceiveActorBeginOverlap`
  (params (OtherActor :type "Actor Object Reference"))
  (bind _asbp_player_character (cast `/Game/Blueprints/Characters/BP_PlayerCharacter` OtherActor))
  (set `/Game/Blueprints/Characters/BP_PlayerCharacter.2xScoreActive` true _asbp_player_character)
  (`KismetSystemLibrary.PrintString` "2X Score Active")
  (bind _aswbp_hud (cast `/Game/UI/HUD/WBP_HUD` (`/Game/Blueprints/Characters/BP_PlayerCharacter.HUD` _asbp_player_character)))
  (`UserWidget.PlayAnimation` _aswbp_hud (`/Game/UI/HUD/WBP_HUD.ItemFadeOut` _aswbp_hud) 0.0 1 "Forward" 1.0 false)
  (`SceneComponent.SetVisibility` (`self.StaticMesh`) false false)
  (`KismetSystemLibrary.Delay` 10.0)
  (bind _asbp_player_character_2 (cast `/Game/Blueprints/Characters/BP_PlayerCharacter` (`GameplayStatics.GetPlayerCharacter` 0)))
  (set `/Game/Blueprints/Characters/BP_PlayerCharacter.2xScoreActive` false _asbp_player_character_2)
  (`KismetSystemLibrary.PrintString` "2X Score Inactive")
  (`self.K2_DestroyActor`))

(fn `UserConstructionScript`)