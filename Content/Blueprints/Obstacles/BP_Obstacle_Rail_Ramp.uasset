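; Rail ramp obstacle that tilts the player for a grind when they enter its left or right trigger.
; Each trigger's begin overlap restarts its own timeline, which blends the player character's current rotation toward opposite fixed angles for each side.
; Every timeline update also applies a strong downward velocity-change impulse through CharacterMovement.
; End-overlap events are empty, so leaving a trigger neither stops the timeline nor restores rotation.
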(event `self.LeftTrigger01.OnComponentBeginOverlap`
  (params (OverlappedComponent :type "PrimitiveComponent Object Reference") (OtherActor :type "Actor Object Reference") (OtherComp :type "PrimitiveComponent Object Reference") (OtherBodyIndex :type Integer) (bFromSweep :type Boolean) (SweepResult :type "HitResult Structure (by ref)"))
  ;[1 1 1] Left Rail Grind
  (bind (_direction _rotate) (`Timeline|Timeline_0` :!via `PlayFromStart`)
    (:`Update`
      (bind _asbp_player_character (cast `/Game/Blueprints/Characters/BP_PlayerCharacter` OtherActor))
      (`self.K2_SetActorRotation` _asbp_player_character (`KismetMathLibrary.RLerp` (`self.K2_GetActorRotation` _asbp_player_character) (struct :`Yaw` 70.0) _rotate) false)
      (`CharacterMovementComponent.AddImpulse` (`Character.CharacterMovement` _asbp_player_character) (0.0 0.0 -3000.0) true))))

(event `self.LeftTrigger01.OnComponentEndOverlap`
  (params (OverlappedComponent :type "PrimitiveComponent Object Reference") (OtherActor :type "Actor Object Reference") (OtherComp :type "PrimitiveComponent Object Reference") (OtherBodyIndex :type Integer))
  ;[1 1 1] Left Rail Grind
)

(event `self.RightTrigger01.OnComponentBeginOverlap`
  (params (OverlappedComponent :type "PrimitiveComponent Object Reference") (OtherActor :type "Actor Object Reference") (OtherComp :type "PrimitiveComponent Object Reference") (OtherBodyIndex :type Integer) (bFromSweep :type Boolean) (SweepResult :type "HitResult Structure (by ref)"))
  ;[1 1 1] Right Rail Grind
  (bind (_direction _rotate) (`Timeline|Timeline_1` :!via `PlayFromStart`)
    (:`Update`
      (bind _asbp_player_character (cast `/Game/Blueprints/Characters/BP_PlayerCharacter` OtherActor))
      (`self.K2_SetActorRotation` _asbp_player_character (`KismetMathLibrary.RLerp` (`self.K2_GetActorRotation` _asbp_player_character) (struct :`Yaw` -70.0) _rotate) false)
      (`CharacterMovementComponent.AddImpulse` (`Character.CharacterMovement` _asbp_player_character) (0.0 0.0 -3000.0) true))))

(event `self.RightTrigger01.OnComponentEndOverlap`
  (params (OverlappedComponent :type "PrimitiveComponent Object Reference") (OtherActor :type "Actor Object Reference") (OtherComp :type "PrimitiveComponent Object Reference") (OtherBodyIndex :type Integer))
  ;[1 1 1] Right Rail Grind
)

(fn `UserConstructionScript`
  (`parent.UserConstructionScript`))