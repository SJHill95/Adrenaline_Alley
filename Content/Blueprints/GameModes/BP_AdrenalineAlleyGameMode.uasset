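; Game mode for Adrenaline Alley that shows the game start screen and signals when the player beats the high score.
; BeginPlay creates the WPB_GameStart widget and adds it to the viewport.
; Every Tick reloads the HighscoreData save slot and compares CurrentPoints with the saved high score.
; The high score sound plays on every frame the points exceed that value, with no one-shot guard.
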(event `self.ReceiveBeginPlay`
  (bind _returnvalue (`|CreateWidget` "/Game/UI/GameStart/WPB_GameStart.WPB_GameStart_C"))
  (`UserWidget.AddToViewport` _returnvalue 0))

(event `self.ReceiveTick`
  (params (DeltaSeconds :type "Float (single-precision)"))
  (bind _returnvalue (`GameplayStatics.LoadGameFromSlot` "HighscoreData"))
  (bind _output_get (set `self.SaverSubClass` _returnvalue))
  (bind _asbp_save_game (cast `/Game/Blueprints/SaveGames/BP_SaveGame` _output_get))
  (if (> (`self.CurrentPoints`) (`/Game/Blueprints/SaveGames/BP_SaveGame.HighscoreValue` _asbp_save_game))
    (`GameplayStatics.PlaySound2D` "/Game/Sounds/SFX/S_Highscore_Cue.S_Highscore_Cue" 1.0 1.0 0.0 null null)))

(fn `UserConstructionScript`)