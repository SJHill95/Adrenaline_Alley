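; BP_SpawnerLocation is a placed spawn point that repeatedly spawns an actor of the Spawner class at its own location.
; Tick waits a random delay between MinDelay and MaxDelay before each spawn.
; It then sets the actor's tick interval to a random value between MinRespawn and MaxRespawn, so spawn timing varies without a separate timer.
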(event `self.ReceiveTick`
  (params (DeltaSeconds :type "Float (single-precision)"))
  (`KismetSystemLibrary.Delay` (`KismetMathLibrary.RandomFloatInRange` (`self.MinDelay`) (`self.MaxDelay`)))
  (bind _output_get (set `self.RespawnTime` (`KismetMathLibrary.RandomFloatInRange` (`self.MinRespawn`) (`self.MaxRespawn`))))
  (`self.SetActorTickInterval` _output_get)
  (`|SpawnActorFromClass` (`self.Spawner`) (`KismetMathLibrary.MakeTransform` (`self.K2_GetActorLocation`)) "Undefined" "OverrideRootScale" null null))

(fn `UserConstructionScript`)