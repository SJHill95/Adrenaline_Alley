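; Endless-runner track tile that fills three lanes on BeginPlay and advances the run when the player crosses its trigger box.
; The overlap has the game mode spawn another tile, adds multiplied points, raises clamped walk speed, then destroys the tile after a delay.
; SpawnObstacles chains lanes, re-rolling at each obstacle or pickup check, so a lane spawning nothing skips later lanes.
; Lane 1's ghost pickup branch is disconnected.
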(event `self.Box.OnComponentBeginOverlap`
  (params (OverlappedComponent :type "PrimitiveComponent Object Reference") (OtherActor :type "Actor Object Reference") (OtherComp :type "PrimitiveComponent Object Reference") (OtherBodyIndex :type Integer) (bFromSweep :type Boolean) (SweepResult :type "HitResult Structure (by ref)"))
  (cast `/Game/Blueprints/Characters/BP_PlayerCharacter` OtherActor)
  (bind _asbp_adrenaline_alley_game_mode (cast `/Game/Blueprints/GameModes/BP_AdrenalineAlleyGameMode` (`GameplayStatics.GetGameMode`)))
  (`/Game/Blueprints/GameModes/BP_AdrenalineAlleyGameMode.SpawnTile` _asbp_adrenaline_alley_game_mode)
  (bind _asbp_adrenaline_alley_game_mode_2 (cast `/Game/Blueprints/GameModes/BP_AdrenalineAlleyGameMode` (`GameplayStatics.GetGameMode`)))
  (set `/Game/Blueprints/GameModes/BP_AdrenalineAlleyGameMode.CurrentPoints` (+ (* 1 (`/Game/Blueprints/GameModes/BP_AdrenalineAlleyGameMode.PointsMultiplier` _asbp_adrenaline_alley_game_mode_2)) (`/Game/Blueprints/GameModes/BP_AdrenalineAlleyGameMode.CurrentPoints` _asbp_adrenaline_alley_game_mode_2)) _asbp_adrenaline_alley_game_mode_2)
  (bind _asbp_player_character (cast `/Game/Blueprints/Characters/BP_PlayerCharacter` (`GameplayStatics.GetPlayerCharacter` 0)))
  (bind _charactermovement (`Character.CharacterMovement` _asbp_player_character))
  (set `CharacterMovementComponent.MaxWalkSpeed` (`KismetMathLibrary.FClamp` (* (`CharacterMovementComponent.MaxWalkSpeed` _charactermovement) 1.01) 1000.0 2000.0) _charactermovement)
  (`KismetSystemLibrary.Delay` 0.5)
  (`self.K2_DestroyActor`))

(event `self.ReceiveBeginPlay`
  (`self.SpawnObstacles`))

(fn `SpawnObstacles`
  (bind _returnvalue (`KismetMathLibrary.RandomFloatInRange` 0.0 1.0))
  (bind _returnvalue_2 (`KismetMathLibrary.RandomFloatInRange` 0.0 1.0))
  (bind _returnvalue_3 (`KismetMathLibrary.RandomFloatInRange` 0.0 1.0))
  (bind _returnvalue_4 (`SceneComponent.K2_GetComponentToWorld` (`self.Lane0`)))
  (bind _returnvalue_5 (`SceneComponent.K2_GetComponentToWorld` (`self.Lane1`)))
  (bind _returnvalue_6 (`SceneComponent.K2_GetComponentToWorld` (`self.Lane2`)))
  ;[1 1 1] Lane 0
  (if (`KismetMathLibrary.InRange_FloatFloat` _returnvalue 0.0 0.2)
    (`|SpawnActorFromClass` "/Game/Blueprints/Obstacles/BP_Obstacle01.BP_Obstacle01_C" _returnvalue_4 "Undefined" "OverrideRootScale" null null)
    ;[1 1 1] Lane 1
    (if (`KismetMathLibrary.InRange_FloatFloat` _returnvalue_3 0.0 0.2) :!label _label
      (`|SpawnActorFromClass` "/Game/Blueprints/Obstacles/BP_Obstacle01.BP_Obstacle01_C" _returnvalue_5 "Undefined" "OverrideRootScale" null null)
      ;[1 1 1] Lane 2
      (if (`KismetMathLibrary.InRange_FloatFloat` _returnvalue_2 0.0 0.2) :!label _label_2
        (`|SpawnActorFromClass` "/Game/Blueprints/Obstacles/BP_Obstacle01.BP_Obstacle01_C" _returnvalue_6 "Undefined" "OverrideRootScale" null null)
        (elif (`KismetMathLibrary.InRange_FloatFloat` _returnvalue_2 0.2 0.3)
          (`|SpawnActorFromClass` "/Game/Blueprints/Obstacles/BP_Obstacle02.BP_Obstacle02_C" _returnvalue_6 "Undefined" "OverrideRootScale" null null)
          (elif (`KismetMathLibrary.InRange_FloatFloat` _returnvalue_2 0.3 0.93)
            (`|SpawnActorFromClass` "/Game/Blueprints/Pickups/BP_Pickup.BP_Pickup_C" _returnvalue_6 "Undefined" "OverrideRootScale" null null)
            (elif (`KismetMathLibrary.InRange_FloatFloat` _returnvalue_2 0.93 0.95)
              (`|SpawnActorFromClass` "/Game/Blueprints/Pickups/BP_MagnetPickup.BP_MagnetPickup_C" _returnvalue_6 "Undefined" "OverrideRootScale" null null)
              (elif (`KismetMathLibrary.InRange_FloatFloat` _returnvalue_2 0.95 0.98)
                (`|SpawnActorFromClass` "/Game/Blueprints/Pickups/BP_DoubleJumpPickup.BP_DoubleJumpPickup_C" _returnvalue_6 "Undefined" "OverrideRootScale" null null)
                (elif (`KismetMathLibrary.InRange_FloatFloat` _returnvalue_2 0.98)
                  (`|SpawnActorFromClass` "/Game/Blueprints/Pickups/BP_GhostPickup.BP_GhostPickup_C" _returnvalue_6 "Undefined" "OverrideRootScale" null null)))))))
      (elif (`KismetMathLibrary.InRange_FloatFloat` _returnvalue_3 0.2 0.3)
        (`|SpawnActorFromClass` "/Game/Blueprints/Obstacles/BP_Obstacle02.BP_Obstacle02_C" _returnvalue_5 "Undefined" "OverrideRootScale" null null)
        (goto _label_2)
        (elif (`KismetMathLibrary.InRange_FloatFloat` _returnvalue_3 0.3 0.93)
          (`|SpawnActorFromClass` "/Game/Blueprints/Pickups/BP_Pickup.BP_Pickup_C" _returnvalue_5 "Undefined" "OverrideRootScale" null null)
          (goto _label_2)
          (elif (`KismetMathLibrary.InRange_FloatFloat` _returnvalue_3 0.93 0.95)
            (`|SpawnActorFromClass` "/Game/Blueprints/Pickups/BP_MagnetPickup.BP_MagnetPickup_C" _returnvalue_5 "Undefined" "OverrideRootScale" null null)
            (goto _label_2)
            (elif (`KismetMathLibrary.InRange_FloatFloat` _returnvalue_3 0.95 0.98)
              (`|SpawnActorFromClass` "/Game/Blueprints/Pickups/BP_DoubleJumpPickup.BP_DoubleJumpPickup_C" _returnvalue_5 "Undefined" "OverrideRootScale" null null)
              (goto _label_2))))))
    (elif (`KismetMathLibrary.InRange_FloatFloat` _returnvalue 0.2 0.3)
      (`|SpawnActorFromClass` "/Game/Blueprints/Obstacles/BP_Obstacle02.BP_Obstacle02_C" _returnvalue_4 "Undefined" "OverrideRootScale" null null)
      (goto _label)
      (elif (`KismetMathLibrary.InRange_FloatFloat` _returnvalue 0.3 0.93)
        (`|SpawnActorFromClass` "/Game/Blueprints/Pickups/BP_Pickup.BP_Pickup_C" _returnvalue_4 "Undefined" "OverrideRootScale" null null)
        (goto _label)
        (elif (`KismetMathLibrary.InRange_FloatFloat` _returnvalue 0.93 0.95)
          (`|SpawnActorFromClass` "/Game/Blueprints/Pickups/BP_MagnetPickup.BP_MagnetPickup_C" _returnvalue_4 "Undefined" "OverrideRootScale" null null)
          (goto _label)
          (elif (`KismetMathLibrary.InRange_FloatFloat` _returnvalue 0.95 0.98)
            (`|SpawnActorFromClass` "/Game/Blueprints/Pickups/BP_DoubleJumpPickup.BP_DoubleJumpPickup_C" _returnvalue_4 "Undefined" "OverrideRootScale" null null)
            (goto _label)
            (elif (`KismetMathLibrary.InRange_FloatFloat` _returnvalue 0.98)
              (`|SpawnActorFromClass` "/Game/Blueprints/Pickups/BP_GhostPickup.BP_GhostPickup_C" _returnvalue_4 "Undefined" "OverrideRootScale" null null)
              (goto _label))))))))

(fn `UserConstructionScript`)