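; Jump boost pickup that, despite its DoubleJump name, raises the player's jump velocity for a limited time.
; On overlap with BP_PlayerCharacter it sets JumpBoostActive, plays the HUD's ItemFadeOut animation, doubles JumpZVelocity and hides its mesh.
; After a ten-second Delay it clears the flag on player character 0, sets a hard-coded normal velocity and destroys itself.
; Collision stays enabled while hidden, and the HUD cast must succeed before velocity changes.
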(event `self.ReceiveActorBeginOverlap`
  (params (OtherActor :type "Actor Object Reference"))
  (bind _asbp_player_character (cast `/Game/Blueprints/Characters/BP_PlayerCharacter` OtherActor))
  (set `/Game/Blueprints/Characters/BP_PlayerCharacter.JumpBoostActive` true _asbp_player_character)
  (bind _aswbp_hud (cast `/Game/UI/HUD/WBP_HUD` (`/Game/Blueprints/Characters/BP_PlayerCharacter.HUD` _asbp_player_character)))
  (`UserWidget.PlayAnimation` _aswbp_hud (`/Game/UI/HUD/WBP_HUD.ItemFadeOut` _aswbp_hud) 0.0 1 "Forward" 1.0 false)
  (set `CharacterMovementComponent.JumpZVelocity` 1000.0 (`Character.CharacterMovement` _asbp_player_character))
  (`SceneComponent.SetVisibility` (`self.StaticMesh`) false false)
  (`KismetSystemLibrary.Delay` 10.0)
  (bind _asbp_player_character_2 (cast `/Game/Blueprints/Characters/BP_PlayerCharacter` (`GameplayStatics.GetPlayerCharacter` 0)))
  (set `/Game/Blueprints/Characters/BP_PlayerCharacter.JumpBoostActive` false _asbp_player_character_2)
  (set `CharacterMovementComponent.JumpZVelocity` 500.0 (`Character.CharacterMovement` _asbp_player_character_2))
  (`self.K2_DestroyActor`))

(fn `UserConstructionScript`)