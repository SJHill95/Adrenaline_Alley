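; BP_Obstacle04 is an obstacle Blueprint that ends the game when the player character hits it.
; It adds its static mesh to the Obstacle array on BeginPlay and calls GhostMode every Tick.
; Overlapping the Trigger calls HitObstacle, then GameOver after a delay, while a separate SlowMoTrigger toggles slow motion as the player enters and leaves.
; GameOver and the construction script only call their parent versions.
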(event `self.ReceiveTick`
  (params (DeltaSeconds :type "Float (single-precision)"))
  ;[1 1 1] Ghost Mode
  (`self.GhostMode`))

(event `self.ReceiveBeginPlay`
  ;[1 1 1] Add obstacles to obstacle array
  (`parent.ReceiveBeginPlay`)
  (`KismetArrayLibrary.Array_Add` (`self.Obstacle`) (`self.StaticMesh`)))

(event `self.Trigger.OnComponentBeginOverlap`
  (params (OverlappedComponent :type "PrimitiveComponent Object Reference") (OtherActor :type "Actor Object Reference") (OtherComp :type "PrimitiveComponent Object Reference") (OtherBodyIndex :type Integer) (bFromSweep :type Boolean) (SweepResult :type "HitResult Structure (by ref)"))
  ;[1 1 1] Game Over trigger
  (cast `/Game/Blueprints/Characters/BP_PlayerCharacter` OtherActor)
  (`self.Hit Obstacle`)
  (`KismetSystemLibrary.Delay` (`self.GameOverDelay`))
  (`self.Game Over`))

(event `self.SlowMoTrigger.OnComponentBeginOverlap`
  (params (OverlappedComponent :type "PrimitiveComponent Object Reference") (OtherActor :type "Actor Object Reference") (OtherComp :type "PrimitiveComponent Object Reference") (OtherBodyIndex :type Integer) (bFromSweep :type Boolean) (SweepResult :type "HitResult Structure (by ref)"))
  ;[1 1 1] Slow Mo Triggers
  (cast `/Game/Blueprints/Characters/BP_PlayerCharacter` OtherActor)
  (`self.SlowMo`))

(event `self.SlowMoTrigger.OnComponentEndOverlap`
  (params (OverlappedComponent :type "PrimitiveComponent Object Reference") (OtherActor :type "Actor Object Reference") (OtherComp :type "PrimitiveComponent Object Reference") (OtherBodyIndex :type Integer))
  ;[1 1 1] Slow Mo Triggers
  (cast `/Game/Blueprints/Characters/BP_PlayerCharacter` OtherActor)
  (`self.SlowMoOff`))

(fn `Game Over`
  (`parent.Game Over`))

(fn `UserConstructionScript`
  (`parent.UserConstructionScript`))