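; BP_MagnetPickup is a timed pickup that grants the player character a magnet power-up.
; On overlap with BP_PlayerCharacter, it sets MagnetActive and hides its Magnet component.
; After a ten-second delay it clears the flag on player 0's character and destroys itself, printing debug messages at both changes.
; The attraction effect itself is not in this Blueprint, which only toggles the flag.
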(event `self.ReceiveBeginPlay`)

(event `self.ReceiveActorBeginOverlap`
  (params (OtherActor :type "Actor Object Reference"))
  (bind _asbp_player_character (cast `/Game/Blueprints/Characters/BP_PlayerCharacter` OtherActor))
  (set `/Game/Blueprints/Characters/BP_PlayerCharacter.MagnetActive` true _asbp_player_character)
  (`KismetSystemLibrary.PrintString` "Magnet Active")
  (`SceneComponent.SetVisibility` (`self.Magnet`) false false)
  (`KismetSystemLibrary.Delay` 10.0)
  (bind _asbp_player_character_2 (cast `/Game/Blueprints/Characters/BP_PlayerCharacter` (`GameplayStatics.GetPlayerCharacter` 0)))
  (set `/Game/Blueprints/Characters/BP_PlayerCharacter.MagnetActive` false _asbp_player_character_2)
  (`KismetSystemLibrary.PrintString` "Magnet Inactive")
  (`self.K2_DestroyActor`))

(fn `UserConstructionScript`)