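; BP_Gold_Coin is a gold coin pickup that awards itself to whatever touches it.
; Overlapping the Coin component sends an AddGoldCoin interface message to that actor and plays the gold score animation on the player's HUD.
; A separate Sphere component does the same for the player character, but only while MagnetActive is set.
; The coin neither moves nor destroys itself in these graphs.
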(event `self.ReceiveActorBeginOverlap`
  (params (OtherActor :type "Actor Object Reference")))

(event `self.Coin.OnComponentBeginOverlap`
  (params (OverlappedComponent :type "PrimitiveComponent Object Reference") (OtherActor :type "Actor Object Reference") (OtherComp :type "PrimitiveComponent Object Reference") (OtherBodyIndex :type Integer) (bFromSweep :type Boolean) (SweepResult :type "HitResult Structure (by ref)"))
  (message `/Game/Blueprints/Coins/CoinPickups.Add_Gold_Coin` OtherActor "")
  (bind _asbp_player_character (cast `/Game/Blueprints/Characters/BP_PlayerCharacter` (`GameplayStatics.GetPlayerCharacter` 0)))
  (bind _hud (`/Game/Blueprints/Characters/BP_PlayerCharacter.HUD` _asbp_player_character))
  (`UserWidget.PlayAnimation` _hud (`/Game/UI/HUD/WBP_HUD.GoldCoinScoreAnimation` _hud) 0.0 1 "Forward" 1.0 false))

(event `self.Sphere.OnComponentBeginOverlap`
  (params (OverlappedComponent :type "PrimitiveComponent Object Reference") (OtherActor :type "Actor Object Reference") (OtherComp :type "PrimitiveComponent Object Reference") (OtherBodyIndex :type Integer) (bFromSweep :type Boolean) (SweepResult :type "HitResult Structure (by ref)"))
  (bind _asbp_player_character (cast `/Game/Blueprints/Characters/BP_PlayerCharacter` OtherActor))
  (if (`/Game/Blueprints/Characters/BP_PlayerCharacter.MagnetActive` _asbp_player_character)
    (message `/Game/Blueprints/Coins/CoinPickups.Add_Gold_Coin` OtherActor "")
    (bind _hud (`/Game/Blueprints/Characters/BP_PlayerCharacter.HUD` _asbp_player_character))
    (`UserWidget.PlayAnimation` _hud (`/Game/UI/HUD/WBP_HUD.GoldCoinScoreAnimation` _hud) 0.0 1 "Forward" 1.0 false)))

(fn `UserConstructionScript`
  (`parent.UserConstructionScript`))