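; Ghost power-up pickup that grants BP_PlayerCharacter a ten-second ghost state on overlap.
; A DoOnce, reset on overlap while ghost is already active, gates the effect: faster walk and level scroll, ghost material, sound and HUD animations, adjusted if magnet is active.
; The pickup hides and moves its mesh away, then reverts the effects after the delay and destroys itself.
; SetParent and ReturnParent store and expose a parent reference.
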(event `self.ReceiveActorBeginOverlap`
  (params (OtherActor :type "Actor Object Reference"))
  (bind _asbp_player_character (cast `/Game/Blueprints/Characters/BP_PlayerCharacter` OtherActor))
  (if (`/Game/Blueprints/Characters/BP_PlayerCharacter.GhostActive` _asbp_player_character)
    (goto _label :!via `Reset`)
    (else
      (`/Engine/EditorBlueprintResources/StandardMacros.DoOnce` false :!label _label
        (:`Completed`
          (set `/Game/Blueprints/Characters/BP_PlayerCharacter.GhostActive` true _asbp_player_character)
          (`SceneComponent.K2_SetWorldLocation` (`self.Ghost`) (0.0 0.0 5000.0) false false)
          (if (`/Game/Blueprints/Characters/BP_PlayerCharacter.MagnetActive` _asbp_player_character)
            (bind _hud (`/Game/Blueprints/Characters/BP_PlayerCharacter.HUD` _asbp_player_character))
            (`UserWidget.PlayAnimation` _hud (`/Game/UI/HUD/WBP_HUD.MoveGhostUI` _hud) 0.0 1 "Forward" 1.0 true))
          (set `CharacterMovementComponent.MaxWalkSpeed` 1000.0 (`Character.CharacterMovement` _asbp_player_character))
          (set `/Game/Blueprints/Game/BP_LevelManager.LevelSpeed` -1000.0 (`/Game/Blueprints/Libraries/BPF_Lib.GetLevelManager`))
          (`UserWidget.PlayAnimation` _hud (`/Game/UI/HUD/WBP_HUD.ItemFadeOut` _hud) 0.0 1 "Forward" 1.0 false)
          (`PrimitiveComponent.SetMaterial` (`Character.Mesh` (`GameplayStatics.GetPlayerCharacter` 0)) 0 "/Game/Materials/Player/M_PlayerGhost.M_PlayerGhost")
          (bind _returnvalue (`GameplayStatics.SpawnSound2D` "/Game/SFX/soundtrack/SFX_Ghost.SFX_Ghost" 1.0 1.0 0.0 null))
          (`SceneComponent.SetVisibility` (`self.Ghost`) false false)
          (`KismetSystemLibrary.Delay` 10.0)
          (bind _asbp_player_character_2 (cast `/Game/Blueprints/Characters/BP_PlayerCharacter` (`GameplayStatics.GetPlayerCharacter` 0)))
          (set `/Game/Blueprints/Characters/BP_PlayerCharacter.GhostActive` false _asbp_player_character_2)
          (`ActorComponent.SetActive` _returnvalue false false)
          (set `CharacterMovementComponent.MaxWalkSpeed` 800.0 (`Character.CharacterMovement` _asbp_player_character_2))
          (set `/Game/Blueprints/Game/BP_LevelManager.LevelSpeed` -800.0 (`/Game/Blueprints/Libraries/BPF_Lib.GetLevelManager`))
          (`PrimitiveComponent.SetMaterial` (`Character.Mesh` (`GameplayStatics.GetPlayerCharacter` 0)) 0 "/Game/Materials/Player/M_Player.M_Player")
          (`self.K2_DestroyActor`))))))

(fn `ReturnParent`
  (returns (Parent :type "/Game/Blueprints/Spawners/BP_SpawnerBase Object Reference"))
  (return (`self.ParentRef`)))

(fn `SetParent`
  (params (Parent :type "/Game/Blueprints/Spawners/BP_SpawnerBase Object Reference"))
  (returns (Return :type Boolean))
  (set `self.ParentRef` Parent)
  (return false))

(fn `UserConstructionScript`)