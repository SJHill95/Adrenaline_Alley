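; BP_Obstacle05 is an obstacle Blueprint, derived from a parent class, that ends the game when the player runs into it.
; Overlap events on its two wall triggers, Wall01Trigger and Wall02Trigger, check for BP_PlayerCharacter and call GameOver.
; GameOver, SpawnCoinsL and the construction script only forward to the parent's implementations, and the default event nodes are disabled.
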(event `self.Wall01Trigger.OnComponentBeginOverlap`
  (params (OverlappedComponent :type "PrimitiveComponent Object Reference") (OtherActor :type "Actor Object Reference") (OtherComp :type "PrimitiveComponent Object Reference") (OtherBodyIndex :type Integer) (bFromSweep :type Boolean) (SweepResult :type "HitResult Structure (by ref)"))
  (cast `/Game/Blueprints/Characters/BP_PlayerCharacter` OtherActor)
  (`self.Game Over`))

(event `self.Wall02Trigger.OnComponentBeginOverlap`
  (params (OverlappedComponent :type "PrimitiveComponent Object Reference") (OtherActor :type "Actor Object Reference") (OtherComp :type "PrimitiveComponent Object Reference") (OtherBodyIndex :type Integer) (bFromSweep :type Boolean) (SweepResult :type "HitResult Structure (by ref)"))
  (cast `/Game/Blueprints/Characters/BP_PlayerCharacter` OtherActor)
  (`self.Game Over`))

(fn `Game Over`
  (`parent.Game Over`))

(fn `SpawnCoinsL`
  (`parent.SpawnCoinsL`))

(fn `UserConstructionScript`
  (`parent.UserConstructionScript`))