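; Base obstacle actor that can spawn gold coins and end the run when the player hits it.
; On BeginPlay, if SpawnCoins is set, random rolls gate spawning five BP_Gold_Coin actors at left or right spawn points.
; GameOver disables mesh collision for a ghosted player, otherwise calls the player's HitObstacle and the level manager's GameOver.
; Its own HitObstacle does a fade and slow-motion effect, and a parent reference has accessors.
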(event `self.ReceiveBeginPlay`
  (bind _returnvalue (`KismetMathLibrary.RandomFloatInRange` 0.0 1.0))
  ;[1 1 1] Spawn Coins
  (if (`self.SpawnCoins`)
    (if (`KismetMathLibrary.InRange_FloatFloat` _returnvalue 0.0 0.5)
      (`self.SpawnCoinsL`)
      (elif (`KismetMathLibrary.InRange_FloatFloat` _returnvalue 0.5)
        (`self.SpawnCoinsR`)))))

(fn `Game Over`
  (bind (_levelmanager _levelmanagerfound) (`/Game/Blueprints/Libraries/BPF_Lib.GetLevelManager`))
  ;[1 1 1] Game Over
  (bind _asbp_player_character (cast `/Game/Blueprints/Characters/BP_PlayerCharacter` (`GameplayStatics.GetPlayerCharacter` 0)))
  (if (`/Game/Blueprints/Characters/BP_PlayerCharacter.GhostActive` _asbp_player_character)
    (`PrimitiveComponent.SetCollisionEnabled` (`self.StaticMesh`) "NoCollision")
    (else
      (`/Game/Blueprints/Characters/BP_PlayerCharacter.HitObstacle` _asbp_player_character)
      (if _levelmanagerfound
        (`/Game/Blueprints/Game/BP_LevelManager.GameOver` _levelmanager)))))

(fn `Hit Obstacle`
  (`PlayerCameraManager.StartCameraFade` (`GameplayStatics.GetPlayerCameraManager` 0) 0.0 1.0 1.0 (struct :`R` 0.744792 :`G` 0.744792 :`B` 0.744792 :`A` 1.0) false true)
  (`GameplayStatics.SetGlobalTimeDilation` 0.2)
  (set `Actor.CustomTimeDilation` 4.0 (`GameplayStatics.GetPlayerCharacter` 0)))

(fn `ReturnParent`
  (returns (Parent :type "/Game/Blueprints/Spawners/BP_SpawnerBase Object Reference"))
  (return (`self.ParentRef`)))

(fn `SetParent`
  (params (Parent :type "/Game/Blueprints/Spawners/BP_SpawnerBase Object Reference"))
  (returns (Return :type Boolean))
  (set `self.ParentRef` Parent)
  (return false))

(fn `SpawnCoinsL`
  (`|ExecutionSequence`
    (:`then_0`
      (set `self.CoinLocation01` (`SceneComponent.K2_GetComponentLocation` (`self.CoinSpawnPoint01_L`)))
      (bind _returnvalue (`|SpawnActorFromClass` "/Game/Blueprints/Coins/BP_Gold_Coin.BP_Gold_Coin_C" (`KismetMathLibrary.MakeTransform` (0.0 0.0 -1000.0)) "Undefined" "OverrideRootScale" null null))
      (`self.K2_SetActorLocation` _returnvalue (`self.CoinLocation01`) false false))
    (:`then_1`
      (set `self.CoinLocation02` (`SceneComponent.K2_GetComponentLocation` (`self.CoinSpawnPoint02_L`)))
      (bind _returnvalue_2 (`|SpawnActorFromClass` "/Game/Blueprints/Coins/BP_Gold_Coin.BP_Gold_Coin_C" (`KismetMathLibrary.MakeTransform` (0.0 0.0 -1000.0)) "Undefined" "OverrideRootScale" null null))
      (`self.K2_SetActorLocation` _returnvalue_2 (`self.CoinLocation02`) false false))
    (:`then_2`
      (set `self.CoinLocation03` (`SceneComponent.K2_GetComponentLocation` (`self.CoinSpawnPoint03_L`)))
      (bind _returnvalue_3 (`|SpawnActorFromClass` "/Game/Blueprints/Coins/BP_Gold_Coin.BP_Gold_Coin_C" (`KismetMathLibrary.MakeTransform` (0.0 0.0 -1000.0)) "Undefined" "OverrideRootScale" null null))
      (`self.K2_SetActorLocation` _returnvalue_3 (`self.CoinLocation03`) false false))
    (:`then_3`
      (set `self.CoinLocation04` (`SceneComponent.K2_GetComponentLocation` (`self.CoinSpawnPoint04_L`)))
      (bind _returnvalue_4 (`|SpawnActorFromClass` "/Game/Blueprints/Coins/BP_Gold_Coin.BP_Gold_Coin_C" (`KismetMathLibrary.MakeTransform` (0.0 0.0 -1000.0)) "Undefined" "OverrideRootScale" null null))
      (`self.K2_SetActorLocation` _returnvalue_4 (`self.CoinLocation04`) false false))
    (:`then_4`
      (set `self.CoinLocation05` (`SceneComponent.K2_GetComponentLocation` (`self.CoinSpawnPoint05_L`)))
      (bind _returnvalue_5 (`|SpawnActorFromClass` "/Game/Blueprints/Coins/BP_Gold_Coin.BP_Gold_Coin_C" (`KismetMathLibrary.MakeTransform` (0.0 0.0 -1000.0)) "Undefined" "OverrideRootScale" null null))
      (`self.K2_SetActorLocation` _returnvalue_5 (`self.CoinLocation05`) false false))))

(fn `SpawnCoinsR`
  (`|ExecutionSequence`
    (:`then_0`
      (set `self.CoinLocation01` (`SceneComponent.K2_GetComponentLocation` (`self.CoinSpawnPoint01_R`)))
      (bind _returnvalue (`|SpawnActorFromClass` "/Game/Blueprints/Coins/BP_Gold_Coin.BP_Gold_Coin_C" (`KismetMathLibrary.MakeTransform` (0.0 0.0 -1000.0)) "Undefined" "OverrideRootScale" null null))
      (`self.K2_SetActorLocation` _returnvalue (`self.CoinLocation01`) false false))
    (:`then_1`
      (set `self.CoinLocation02` (`SceneComponent.K2_GetComponentLocation` (`self.CoinSpawnPoint02_R`)))
      (bind _returnvalue_2 (`|SpawnActorFromClass` "/Game/Blueprints/Coins/BP_Gold_Coin.BP_Gold_Coin_C" (`KismetMathLibrary.MakeTransform` (0.0 0.0 -1000.0)) "Undefined" "OverrideRootScale" null null))
      (`self.K2_SetActorLocation` _returnvalue_2 (`self.CoinLocation02`) false false))
    (:`then_2`
      (set `self.CoinLocation03` (`SceneComponent.K2_GetComponentLocation` (`self.CoinSpawnPoint03_R`)))
      (bind _returnvalue_3 (`|SpawnActorFromClass` "/Game/Blueprints/Coins/BP_Gold_Coin.BP_Gold_Coin_C" (`KismetMathLibrary.MakeTransform` (0.0 0.0 -1000.0)) "Undefined" "OverrideRootScale" null null))
      (`self.K2_SetActorLocation` _returnvalue_3 (`self.CoinLocation03`) false false))
    (:`then_3`
      (set `self.CoinLocation04` (`SceneComponent.K2_GetComponentLocation` (`self.CoinSpawnPoint04_R`)))
      (bind _returnvalue_4 (`|SpawnActorFromClass` "/Game/Blueprints/Coins/BP_Gold_Coin.BP_Gold_Coin_C" (`KismetMathLibrary.MakeTransform` (0.0 0.0 -1000.0)) "Undefined" "OverrideRootScale" null null))
      (`self.K2_SetActorLocation` _returnvalue_4 (`self.CoinLocation04`) false false))
    (:`then_4`
      (set `self.CoinLocation05` (`SceneComponent.K2_GetComponentLocation` (`self.CoinSpawnPoint05_R`)))
      (bind _returnvalue_5 (`|SpawnActorFromClass` "/Game/Blueprints/Coins/BP_Gold_Coin.BP_Gold_Coin_C" (`KismetMathLibrary.MakeTransform` (0.0 0.0 -1000.0)) "Undefined" "OverrideRootScale" null null))
      (`self.K2_SetActorLocation` _returnvalue_5 (`self.CoinLocation05`) false false))))

(fn `UserConstructionScript`)