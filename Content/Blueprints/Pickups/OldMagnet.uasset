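; Magnet pickup Blueprint that grants the player character a timed magnet power-up on overlap.
; A DoOnce gate fires when the magnet is inactive and resets if it is already active.
; Activation sets the player's MagnetActive flag, plays the HUD item fade-out and hides the magnet.
; After the MagnetTimer delay, it clears the flag and destroys itself, with debug prints for both states.
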(event `self.ReceiveActorBeginOverlap`
  (params (OtherActor :type "Actor Object Reference"))
  ;[1 1 1] Pickup
  (bind _asbp_player_character (cast `/Game/Blueprints/Characters/BP_PlayerCharacter` OtherActor))
  (if (`/Game/Blueprints/Characters/BP_PlayerCharacter.MagnetActive` _asbp_player_character)
    (goto _label :!via `Reset`)
    (else
      (`/Engine/EditorBlueprintResources/StandardMacros.DoOnce` false :!label _label
        (:`Completed`
          (set `/Game/Blueprints/Characters/BP_PlayerCharacter.MagnetActive` true _asbp_player_character)
          (bind _hud (`/Game/Blueprints/Characters/BP_PlayerCharacter.HUD` _asbp_player_character))
          (`UserWidget.PlayAnimation` _hud (`/Game/UI/HUD/WBP_HUD.ItemFadeOut` _hud) 0.0 1 "Forward" 1.0 false)
          (`KismetSystemLibrary.PrintString` "Magnet Active")
          (`SceneComponent.SetVisibility` (`self.Magnet`) false false)
          (`KismetSystemLibrary.Delay` (`self.MagnetTimer`))
          (bind _asbp_player_character_2 (cast `/Game/Blueprints/Characters/BP_PlayerCharacter` (`GameplayStatics.GetPlayerCharacter` 0)))
          (set `/Game/Blueprints/Characters/BP_PlayerCharacter.MagnetActive` false _asbp_player_character_2)
          (`KismetSystemLibrary.PrintString` "Magnet Inactive")
          (`self.K2_DestroyActor`))))))

(event `self.ReceiveActorEndOverlap`
  (params (OtherActor :type "Actor Object Reference")))

(fn `UserConstructionScript`)