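; Base spawner Blueprint that creates actors from configurable classes far below the origin and passes itself to each as parent through SetParentMessage.
; SpawnItem picks among three classes by chained random range checks, re-rolling at each check, so it can spawn nothing.
; SpawnActor sequences the first two classes into a shared return.
; SpawnedActorHitBounds is an empty hook receiving an out-of-bounds actor.
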(fn `SpawnActor`
  (returns (ReturnValue :type "Actor Object Reference"))
  (`|ExecutionSequence`
    (:`then_0`
      (bind _returnvalue (`|SpawnActorFromClass` (`self.SpawnActorType`) (`KismetMathLibrary.MakeTransform` (0.0 0.0 -1000.0)) "Undefined" "OverrideRootScale" null null))
      (message `/Game/Blueprints/Misc/BPI_Spawnable.SetParent` _returnvalue self))
    (:`then_1`
      (bind _returnvalue_2 (`|SpawnActorFromClass` (`self.SpawnActor02`) (`KismetMathLibrary.MakeTransform` (0.0 0.0 -1000.0)) "Undefined" "OverrideRootScale" null null))
      (message `/Game/Blueprints/Misc/BPI_Spawnable.SetParent` _returnvalue_2 self)))
  (return _returnvalue))

(fn `SpawnedActorHitBounds`
  (params (OutOfBoundsActor :type "Actor Object Reference")))

(fn `SpawnItem`
  (returns (ReturnValue :type "Actor Object Reference"))
  (bind _returnvalue (`KismetMathLibrary.RandomFloatInRange` 0.0 1.0))
  (if (`KismetMathLibrary.InRange_FloatFloat` _returnvalue 0.0 0.6)
    (bind _returnvalue_2 (`|SpawnActorFromClass` (`self.SpawnActorType`) (`KismetMathLibrary.MakeTransform` (0.0 0.0 -1000.0)) "Undefined" "OverrideRootScale" null null))
    (message `/Game/Blueprints/Misc/BPI_Spawnable.SetParent` _returnvalue_2 self)
    (return _returnvalue_2)
    (elif (`KismetMathLibrary.InRange_FloatFloat` _returnvalue 0.6 0.8)
      (bind _returnvalue_3 (`|SpawnActorFromClass` (`self.SpawnActor02`) (`KismetMathLibrary.MakeTransform` (0.0 0.0 -1000.0)) "Undefined" "OverrideRootScale" null null))
      (message `/Game/Blueprints/Misc/BPI_Spawnable.SetParent` _returnvalue_3 self)
      (return _returnvalue_3)
      (elif (`KismetMathLibrary.InRange_FloatFloat` _returnvalue 0.8)
        (bind _returnvalue_4 (`|SpawnActorFromClass` (`self.SpawnActor03`) (`KismetMathLibrary.MakeTransform` (0.0 0.0 -1000.0)) "Undefined" "OverrideRootScale" null null))
        (message `/Game/Blueprints/Misc/BPI_Spawnable.SetParent` _returnvalue_4 self)
        (return _returnvalue_4)))))

(fn `UserConstructionScript`)