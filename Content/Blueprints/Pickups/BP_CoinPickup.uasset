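; Coin pickup that adds to the game mode's Pickup count, plays a sound and destroys itself when the player touches it.
; A Sphere overlap handles magnet collection when the player's MagnetActive is set, flagging the coin Used so direct contact cannot count it again.
; It then counts and destroys the coin after a short delay, while a timeline pulls it toward the player using VInterpTo plus a Slide offset.
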(event `self.Coin.OnComponentBeginOverlap`
  (params (OverlappedComponent :type "PrimitiveComponent Object Reference") (OtherActor :type "Actor Object Reference") (OtherComp :type "PrimitiveComponent Object Reference") (OtherBodyIndex :type Integer) (bFromSweep :type Boolean) (SweepResult :type "HitResult Structure (by ref)"))
  (cast `/Game/Blueprints/Characters/BP_PlayerCharacter` OtherActor)
  (bind _asbp_adrenaline_alley_game_mode (cast `/Game/Blueprints/GameModes/BP_AdrenalineAlleyGameMode` (`GameplayStatics.GetGameMode`)))
  (if (not (`self.Used`))
    (`/Engine/EditorBlueprintResources/StandardMacros.IncrementInt` (`/Game/Blueprints/GameModes/BP_AdrenalineAlleyGameMode.Pickup` _asbp_adrenaline_alley_game_mode)
      (:`  `
        (`GameplayStatics.PlaySound2D` "/Game/SFX/SFX_CoinPickup.SFX_CoinPickup" 1.0 1.0 0.0 null null)
        (`self.K2_DestroyActor`)))))

(event `self.ReceiveActorBeginOverlap`
  (params (OtherActor :type "Actor Object Reference")))

(event `self.Sphere.OnComponentBeginOverlap`
  (params (OverlappedComponent :type "PrimitiveComponent Object Reference") (OtherActor :type "Actor Object Reference") (OtherComp :type "PrimitiveComponent Object Reference") (OtherBodyIndex :type Integer) (bFromSweep :type Boolean) (SweepResult :type "HitResult Structure (by ref)"))
  (bind _asbp_player_character (cast `/Game/Blueprints/Characters/BP_PlayerCharacter` OtherActor))
  (if (`/Game/Blueprints/Characters/BP_PlayerCharacter.MagnetActive` _asbp_player_character)
    (`|ExecutionSequence`
      (:`then_0`
        (bind _asbp_adrenaline_alley_game_mode (cast `/Game/Blueprints/GameModes/BP_AdrenalineAlleyGameMode` (`GameplayStatics.GetGameMode`)))
        (set `self.Used` true)
        (`GameplayStatics.PlaySound2D` "/Game/SFX/SFX_CoinPickup.SFX_CoinPickup" 1.0 1.0 0.0 null null)
        (`KismetSystemLibrary.Delay` 0.3)
        (`/Engine/EditorBlueprintResources/StandardMacros.IncrementInt` (`/Game/Blueprints/GameModes/BP_AdrenalineAlleyGameMode.Pickup` _asbp_adrenaline_alley_game_mode)
          (:`  `
            (`self.K2_DestroyActor`))))
      (:`then_1`
        (bind (_direction _slide) (`Timeline|Timeline_0`)
          (:`Update`
            (`self.K2_SetActorLocation` (+ _slide (`KismetMathLibrary.VInterpTo` (.location (`self.GetTransform`)) (`self.K2_GetActorLocation` (`GameplayStatics.GetPlayerCharacter` 0)) (`GameplayStatics.GetWorldDeltaSeconds`) 15.0)))))))))

(fn `UserConstructionScript`)