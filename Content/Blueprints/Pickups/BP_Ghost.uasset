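; Ghost power-up pickup that spins in place and puts the player into a timed ghost state on overlap.
; Activation raises walk and level scroll speed, swaps the mesh to a ghost material, plays sound and HUD fade, and moves the pickup away.
; A DoOnce gated by the player's GhostActive flag guards activation.
; After a delay it restores speeds and hard-coded original materials, deactivates the sound and destroys itself.
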(event `self.ReceiveTick`
  (params (DeltaSeconds :type "Float (single-precision)"))
  ;[1 1 1] Rotation
  (`SceneComponent.K2_AddLocalRotation` (`self.Ghost`) (`KismetMathLibrary.MakeRotator` 0.0 0.0 (* DeltaSeconds (`self.YawPerSecond`))) false false))

(event `self.ReceiveActorBeginOverlap`
  (params (OtherActor :type "Actor Object Reference"))
  (bind _mesh (`Character.Mesh` (`GameplayStatics.GetPlayerCharacter` 0)))
  (bind _asbp_player_character (cast `/Game/Blueprints/Characters/BP_PlayerCharacter` OtherActor))
  (if (`/Game/Blueprints/Characters/BP_PlayerCharacter.GhostActive` _asbp_player_character)
    (goto _label :!via `Reset`)
    (else
      (`/Engine/EditorBlueprintResources/StandardMacros.DoOnce` false :!label _label
        (:`Completed`
          (set `/Game/Blueprints/Characters/BP_PlayerCharacter.GhostActive` true _asbp_player_character)
          (`KismetSystemLibrary.PrintString` "Ghost Active")
          (`SceneComponent.K2_SetWorldLocation` (`self.Ghost`) (0.0 0.0 5000.0) false false)
          (set `CharacterMovementComponent.MaxWalkSpeed` 1000.0 (`Character.CharacterMovement` _asbp_player_character))
          (set `/Game/Blueprints/Game/BP_LevelManager.LevelSpeed` -1000.0 (`/Game/Blueprints/Libraries/BPF_Lib.GetLevelManager`))
          (bind _hud (`/Game/Blueprints/Characters/BP_PlayerCharacter.HUD` _asbp_player_character))
          (`UserWidget.PlayAnimation` _hud (`/Game/UI/HUD/WBP_HUD.ItemFadeOut` _hud) 0.0 1 "Forward" 1.0 false)
          (for _index (range 13)
            (`PrimitiveComponent.SetMaterial` (`Character.Mesh` (`GameplayStatics.GetPlayerCharacter` 0)) _index "/Game/Materials/Player/M_PlayerGhost.M_PlayerGhost")
            (bind _returnvalue (`GameplayStatics.SpawnSound2D` "/Game/Sounds/soundtrack/SFX_Ghost.SFX_Ghost" 1.0 1.0 0.0 null false false))
            (`SceneComponent.SetVisibility` (`self.Ghost`) false false)
            (`KismetSystemLibrary.Delay` 10.0)
            (bind _asbp_player_character_2 (cast `/Game/Blueprints/Characters/BP_PlayerCharacter` (`GameplayStatics.GetPlayerCharacter` 0)))
            (set `/Game/Blueprints/Characters/BP_PlayerCharacter.GhostActive` false _asbp_player_character_2)
            (`ActorComponent.SetActive` _returnvalue false false)
            (set `CharacterMovementComponent.MaxWalkSpeed` 800.0 (`Character.CharacterMovement` _asbp_player_character_2))
            (set `/Game/Blueprints/Game/BP_LevelManager.LevelSpeed` -800.0 (`/Game/Blueprints/Libraries/BPF_Lib.GetLevelManager`))
            (`PrimitiveComponent.SetMaterial` _mesh 12 "/Game/Materials/Player/Character/M_Shoe_Soles.M_Shoe_Soles")
            (`PrimitiveComponent.SetMaterial` _mesh 11 "/Game/Materials/Player/Character/M_Shoes.M_Shoes")
            (`PrimitiveComponent.SetMaterial` _mesh 10 "/Game/Materials/Player/Character/M_Hair.M_Hair")
            (`PrimitiveComponent.SetMaterial` _mesh 9 "/Game/Materials/Player/Character/M_Helmet.M_Helmet")
            (`PrimitiveComponent.SetMaterial` _mesh 8 "/Game/Materials/Player/Character/M_Pants.M_Pants")
            (`PrimitiveComponent.SetMaterial` _mesh 7 "/Game/Materials/Player/Character/M_Hoodie.M_Hoodie")
            (`PrimitiveComponent.SetMaterial` _mesh 6 "/Game/Materials/Player/Character/M_Mouth.M_Mouth")
            (`PrimitiveComponent.SetMaterial` _mesh 5 "/Game/Materials/Player/Character/M_Skin.M_Skin")
            (`PrimitiveComponent.SetMaterial` _mesh 4 "/Game/Materials/Player/Character/M_Eyebrows.M_Eyebrows")
            (`PrimitiveComponent.SetMaterial` _mesh 3 "/Game/Materials/Player/Character/M_Eye.M_Eye")
            (`PrimitiveComponent.SetMaterial` _mesh 2 "/Game/Materials/Player/Character/M_Iris02.M_Iris02")
            (`PrimitiveComponent.SetMaterial` _mesh 1 "/Game/Materials/Player/Character/M_Iris.M_Iris")
            (`PrimitiveComponent.SetMaterial` _mesh 0 "/Game/Materials/Player/Character/M_Pupil.M_Pupil")
            (`self.K2_DestroyActor`)))))))

(fn `ReturnParent`
  (returns (Parent :type "/Game/Blueprints/Spawners/BP_SpawnerBase Object Reference"))
  (return (`self.ParentRef`)))

(fn `SetParent`
  (params (Parent :type "/Game/Blueprints/Spawners/BP_SpawnerBase Object Reference"))
  (returns (Return :type Boolean))
  (set `self.ParentRef` Parent)
  (return false))

(fn `UserConstructionScript`)