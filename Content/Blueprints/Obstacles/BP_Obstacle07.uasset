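; BP_Obstacle07 is an obstacle with a randomly placed mini ramp, a jump boost zone and a game-over foam pit.
; BeginPlay moves the ramp to a shuffled right, middle or left spawn, then optionally spawns gold coins at five points after a delay.
; The boost trigger toggles the player's slow-mo and calls the level manager's JumpBoost on entry and exit.
; Player overlap with the foam pit calls HitObstacle, then GameOver after a delay.
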(event `self.ReceiveBeginPlay`
  (bind _spawns (`self.Spawns`))
  ;[0.5637 0.7578 1] Spawn Mini Ramp
  (`parent.ReceiveBeginPlay`)
  (for _index (range 3)
    (`KismetArrayLibrary.Array_Add` _spawns (select `int` _index :`0` (`self.RightSpawn`) :`1` (`self.MiddleSpawn`) :`2` (`self.LeftSpawn`)))
    (`KismetArrayLibrary.Array_Shuffle` _spawns)
    (`SceneComponent.K2_SetWorldLocation` (`self.MiniRamp`) (`SceneComponent.K2_GetComponentLocation` (`|GetArrayItem` (`self.Spawns`))) false false)
    (`KismetSystemLibrary.Delay` 1.0)
    (if (`self.bSpawnCoinsOb07`)
      (for _index_2 (range 5)
        (`KismetArrayLibrary.Array_Add` (`self.CoinSpawns`) (select `int` _index_2 :`0` (`self.CoinSpawnPoint01`) :`1` (`self.CoinSpawnPoint02`) :`2` (`self.CoinSpawnPoint03`) :`3` (`self.CoinSpawnPoint04`) :`4` (`self.CoinSpawnPoint05`)))
        (`|SpawnActorFromClass` "/Game/Blueprints/Coins/BP_Gold_Coin.BP_Gold_Coin_C" (`KismetMathLibrary.MakeTransform` (`SceneComponent.K2_GetComponentLocation` (`|GetArrayItem` (`self.CoinSpawns`) _index_2))) "Undefined" "OverrideRootScale" null null)))))

(event `self.FoamPitTrigger.OnComponentBeginOverlap`
  (params (OverlappedComponent :type "PrimitiveComponent Object Reference") (OtherActor :type "Actor Object Reference") (OtherComp :type "PrimitiveComponent Object Reference") (OtherBodyIndex :type Integer) (bFromSweep :type Boolean) (SweepResult :type "HitResult Structure (by ref)"))
  ;[1 0.08854 0.08854] FoamPit GameOver trigger
  (cast `/Game/Characters/BP_PlayerCharacter` OtherActor)
  (`self.Hit Obstacle`)
  (`KismetSystemLibrary.Delay` (`self.GameOverDelay`))
  (`self.Game Over`))

(event `self.JumpBoostTrigger.OnComponentBeginOverlap`
  (params (OverlappedComponent :type "PrimitiveComponent Object Reference") (OtherActor :type "Actor Object Reference") (OtherComp :type "PrimitiveComponent Object Reference") (OtherBodyIndex :type Integer) (bFromSweep :type Boolean) (SweepResult :type "HitResult Structure (by ref)"))
  ;[0.5422 1 0.386] Jump Boost Trigger
  (bind _asbp_player_character (cast `/Game/Characters/BP_PlayerCharacter` OtherActor))
  (set `/Game/Characters/BP_PlayerCharacter.SlowMoActive` true _asbp_player_character)
  (bind _asbp_level_manager (cast `/Game/Blueprints/Game/BP_LevelManager` (`/Game/Blueprints/Libraries/BPF_Lib.GetLevelManager`)))
  (`/Game/Blueprints/Game/BP_LevelManager.JumpBoost` _asbp_level_manager))

(event `self.JumpBoostTrigger.OnComponentEndOverlap`
  (params (OverlappedComponent :type "PrimitiveComponent Object Reference") (OtherActor :type "Actor Object Reference") (OtherComp :type "PrimitiveComponent Object Reference") (OtherBodyIndex :type Integer))
  ;[0.5422 1 0.386] Jump Boost Trigger
  (bind _asbp_player_character (cast `/Game/Characters/BP_PlayerCharacter` OtherActor))
  (set `/Game/Characters/BP_PlayerCharacter.SlowMoActive` false _asbp_player_character)
  (bind _asbp_level_manager (cast `/Game/Blueprints/Game/BP_LevelManager` (`/Game/Blueprints/Libraries/BPF_Lib.GetLevelManager`)))
  (`/Game/Blueprints/Game/BP_LevelManager.JumpBoost` _asbp_level_manager))

(fn `UserConstructionScript`
  (`parent.UserConstructionScript`))