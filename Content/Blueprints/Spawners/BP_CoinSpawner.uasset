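; BP_CoinSpawner is a one-shot spawner that places a random coin at its own location on BeginPlay, then destroys itself after a SpawnRate delay.
; SpawnItems spawns a Coin on about half of rolls, otherwise rolls again for a SilverCoin, so roughly a quarter of spawners produce nothing.
; An unconnected third Coin branch in SpawnItems never runs.
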(event `self.ReceiveBeginPlay`
  (`self.SpawnItems`)
  (`KismetSystemLibrary.Delay` (`self.SpawnRate`))
  (`self.K2_DestroyActor`))

(fn `SpawnItems`
  (bind _returnvalue (`KismetMathLibrary.RandomFloatInRange` 0.0 1.0))
  (if (`KismetMathLibrary.InRange_FloatFloat` _returnvalue 0.0 0.5)
    (`|SpawnActorFromClass` (`self.Coin`) (`KismetMathLibrary.MakeTransform` (`self.K2_GetActorLocation`)) "Undefined" "OverrideRootScale" null null)
    (elif (`KismetMathLibrary.InRange_FloatFloat` _returnvalue 0.5)
      (`|SpawnActorFromClass` (`self.SilverCoin`) (`KismetMathLibrary.MakeTransform` (`self.K2_GetActorLocation`)) "Undefined" "OverrideRootScale" null null))))

(fn `UserConstructionScript`)