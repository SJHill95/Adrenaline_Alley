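; A pickup that grants the player a temporary ghost state on overlap.
; It sets GhostActive on BP_PlayerCharacter, plays the HUD's ItemFadeOut animation, swaps the player mesh to a ghost material and hides its own mesh.
; After a fixed delay it clears the flag, restores the normal material via player character 0 and destroys itself.
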(event `self.ReceiveActorBeginOverlap`
  (params (OtherActor :type "Actor Object Reference"))
  (bind _asbp_player_character (cast `/Game/Blueprints/Characters/BP_PlayerCharacter` OtherActor))
  (set `/Game/Blueprints/Characters/BP_PlayerCharacter.GhostActive` true _asbp_player_character)
  (bind _aswbp_hud (cast `/Game/UI/HUD/WBP_HUD` (`/Game/Blueprints/Characters/BP_PlayerCharacter.HUD` _asbp_player_character)))
  (`UserWidget.PlayAnimation` _aswbp_hud (`/Game/UI/HUD/WBP_HUD.ItemFadeOut` _aswbp_hud) 0.0 1 "Forward" 1.0 false)
  (`PrimitiveComponent.SetMaterial` (`Character.Mesh` (`GameplayStatics.GetPlayerCharacter` 0)) 0 "/Game/Materials/Player/M_PlayerGhost.M_PlayerGhost")
  (`SceneComponent.SetVisibility` (`self.StaticMesh`) false false)
  (`KismetSystemLibrary.Delay` 10.0)
  (bind _asbp_player_character_2 (cast `/Game/Blueprints/Characters/BP_PlayerCharacter` (`GameplayStatics.GetPlayerCharacter` 0)))
  (set `/Game/Blueprints/Characters/BP_PlayerCharacter.GhostActive` false _asbp_player_character_2)
  (`PrimitiveComponent.SetMaterial` (`Character.Mesh` (`GameplayStatics.GetPlayerCharacter` 0)) 0 "/Game/Materials/Player/M_Player.M_Player")
  (`self.K2_DestroyActor`))

(fn `UserConstructionScript`)