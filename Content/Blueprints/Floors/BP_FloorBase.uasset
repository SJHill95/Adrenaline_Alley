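; Base floor Blueprint that offers randomized decal materials and keeps a reference to the spawner set as its parent.
; RandomMaterial and RandomPlatformMaterial choose between two materials for the wall and platform decals, making a fresh random roll for the second option, so a decal can stay unchanged.
; SetParent and ReturnParent store and expose ParentSpawner.
; BeginPlay and the construction script are empty, so nothing here calls the randomizers.
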(event `self.ReceiveBeginPlay`)

(fn `Random Material`
  (bind _returnvalue (`KismetMathLibrary.RandomFloatInRange` 0.0 1.0))
  (if (`KismetMathLibrary.InRange_FloatFloat` _returnvalue 0.0 0.5)
    (`PrimitiveComponent.SetMaterial` (`self.WallDecal`) 0 "/Game/Materials/Walls/M_Wall.M_Wall")
    (elif (`KismetMathLibrary.InRange_FloatFloat` _returnvalue 0.5)
      (`PrimitiveComponent.SetMaterial` (`self.WallDecal`) 0 "/Game/Materials/Walls/M_Wall_R.M_Wall_R"))))

(fn `Random Platform Material`
  (bind _returnvalue (`KismetMathLibrary.RandomFloatInRange` 0.0 1.0))
  (if (`KismetMathLibrary.InRange_FloatFloat` _returnvalue 0.0 0.3)
    (`PrimitiveComponent.SetMaterial` (`self.PlatformDecal`) 0 "/Game/Materials/Walls/M_Platform_Text.M_Platform_Text")
    (elif (`KismetMathLibrary.InRange_FloatFloat` _returnvalue 0.3)
      (`PrimitiveComponent.SetMaterial` (`self.PlatformDecal`) 0 "/Game/Materials/Walls/M_Platform.M_Platform"))))

(fn `ReturnParent`
  (returns (Parent :type "/Game/Blueprints/Spawners/BP_SpawnerBase Object Reference"))
  (return (`self.ParentSpawner`)))

(fn `SetParent`
  (params (Parent :type "/Game/Blueprints/Spawners/BP_SpawnerBase Object Reference"))
  (returns (Return :type Boolean))
  (set `self.ParentSpawner` Parent))

(fn `UserConstructionScript`)