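; BP_MainGameMusic plays the main game's background music and mutes it while the player is in ghost mode.
; On BeginPlay it spawns the SFX_MainGame_Cue as a 2D sound and keeps the audio component.
; Every Tick it casts the player character to BP_PlayerCharacter and pauses or resumes the music based on its GhostActive flag.
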(event `self.ReceiveBeginPlay`
  (bind _returnvalue (`GameplayStatics.SpawnSound2D` "/Game/Sounds/SFX_MainGame_Cue.SFX_MainGame_Cue" 1.0 1.0 0.0 null))
  (set `self.Music` _returnvalue))

(event `self.ReceiveTick`
  (params (DeltaSeconds :type "Float (single-precision)"))
  (bind _asbp_player_character (cast `/Game/Blueprints/Characters/BP_PlayerCharacter` (`GameplayStatics.GetPlayerCharacter` 0)))
  (if (`/Game/Blueprints/Characters/BP_PlayerCharacter.GhostActive` _asbp_player_character)
    (`AudioComponent.SetPaused` (`self.Music`) true)
    (else
      (`AudioComponent.SetPaused` (`self.Music`) false))))

(fn `UserConstructionScript`)