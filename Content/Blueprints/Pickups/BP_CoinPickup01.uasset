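; Coin pickup that adds points and a pickup count to the Adrenaline Alley game mode when the player collects it.
; Touching the coin plays a sound and HUD score animation, briefly flags CoinPickedUp on the player, then destroys the actor.
; With the player's magnet active, the outer sphere marks it Used, blocking double collection, and awards it after a short delay while a timeline pulls the rescaled coin toward the player.
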(event `self.Coin.OnComponentBeginOverlap`
  (params (OverlappedComponent :type "PrimitiveComponent Object Reference") (OtherActor :type "Actor Object Reference") (OtherComp :type "PrimitiveComponent Object Reference") (OtherBodyIndex :type Integer) (bFromSweep :type Boolean) (SweepResult :type "HitResult Structure (by ref)"))
  ;[1 1 1] Coin points, animation and sound
  (cast `/Game/Blueprints/Characters/BP_PlayerCharacter` OtherActor)
  (bind _asbp_adrenaline_alley_game_mode (cast `/Game/Blueprints/GameModes/BP_AdrenalineAlleyGameMode` (`GameplayStatics.GetGameMode`)))
  (bind _asbp_player_character (cast `/Game/Blueprints/Characters/BP_PlayerCharacter` (`GameplayStatics.GetPlayerCharacter` 0)))
  (if (not (`self.Used`))
    (`/Engine/EditorBlueprintResources/StandardMacros.IncrementInt` (`/Game/Blueprints/GameModes/BP_AdrenalineAlleyGameMode.Pickup` _asbp_adrenaline_alley_game_mode)
      (:`  `
        (set `/Game/Blueprints/GameModes/BP_AdrenalineAlleyGameMode.CurrentPoints` (+ (`/Game/Blueprints/GameModes/BP_AdrenalineAlleyGameMode.CurrentPoints` _asbp_adrenaline_alley_game_mode) (`self.CoinPoints`)) _asbp_adrenaline_alley_game_mode)
        (set `/Game/Blueprints/Characters/BP_PlayerCharacter.CoinPickedUp` true _asbp_player_character)
        (`GameplayStatics.PlaySound2D` "/Game/SFX/SFX_CoinPickup.SFX_CoinPickup" 1.0 1.0 0.0 null null)
        (`SceneComponent.SetVisibility` (`self.Coin`) false false)
        (bind _asbp_player_character_2 (cast `/Game/Blueprints/Characters/BP_PlayerCharacter` (`GameplayStatics.GetPlayerCharacter` 0)))
        (bind _hud (`/Game/Blueprints/Characters/BP_PlayerCharacter.HUD` _asbp_player_character_2))
        (`UserWidget.PlayAnimation` _hud (`/Game/UI/HUD/WBP_HUD.CoinScoreAnimation` _hud) 0.0 1 "Forward" 1.0 false)
        (`KismetSystemLibrary.Delay` 0.8)
        (set `/Game/Blueprints/Characters/BP_PlayerCharacter.CoinPickedUp` false _asbp_player_character)
        (`self.K2_DestroyActor`)))))

(event `self.Sphere.OnComponentBeginOverlap`
  (params (OverlappedComponent :type "PrimitiveComponent Object Reference") (OtherActor :type "Actor Object Reference") (OtherComp :type "PrimitiveComponent Object Reference") (OtherBodyIndex :type Integer) (bFromSweep :type Boolean) (SweepResult :type "HitResult Structure (by ref)"))
  (bind (_returnvalue_x _returnvalue_y _returnvalue_z) (`KismetMathLibrary.BreakVector` (`self.K2_GetActorLocation` (`GameplayStatics.GetPlayerCharacter` 0))))
  ;[1 1 1] Magnet
  (bind _asbp_player_character (cast `/Game/Blueprints/Characters/BP_PlayerCharacter` OtherActor))
  (if (`/Game/Blueprints/Characters/BP_PlayerCharacter.MagnetActive` _asbp_player_character)
    (`|ExecutionSequence`
      (:`then_0`
        (bind _asbp_adrenaline_alley_game_mode (cast `/Game/Blueprints/GameModes/BP_AdrenalineAlleyGameMode` (`GameplayStatics.GetGameMode`)))
        (set `self.Used` true)
        (`GameplayStatics.PlaySound2D` "/Game/SFX/SFX_CoinPickup.SFX_CoinPickup" 1.0 1.0 0.0 null null)
        (`KismetSystemLibrary.Delay` 0.3)
        (`/Engine/EditorBlueprintResources/StandardMacros.IncrementInt` (`/Game/Blueprints/GameModes/BP_AdrenalineAlleyGameMode.Pickup` _asbp_adrenaline_alley_game_mode)
          (:`  `
            (set `/Game/Blueprints/GameModes/BP_AdrenalineAlleyGameMode.CurrentPoints` (+ (`/Game/Blueprints/GameModes/BP_AdrenalineAlleyGameMode.CurrentPoints` _asbp_adrenaline_alley_game_mode) (`self.CoinPoints`)) _asbp_adrenaline_alley_game_mode)
            (bind _asbp_player_character_2 (cast `/Game/Blueprints/Characters/BP_PlayerCharacter` (`GameplayStatics.GetPlayerCharacter` 0)))
            (`SceneComponent.SetVisibility` (`self.Coin`) false false)
            (set `/Game/Blueprints/Characters/BP_PlayerCharacter.CoinPickedUp` true _asbp_player_character_2)
            (bind _hud (`/Game/Blueprints/Characters/BP_PlayerCharacter.HUD` _asbp_player_character_2))
            (`UserWidget.PlayAnimation` _hud (`/Game/UI/HUD/WBP_HUD.CoinScoreAnimation` _hud) 0.0 1 "Forward" 1.0 false)
            (`KismetSystemLibrary.Delay` 0.8)
            (set `/Game/Blueprints/Characters/BP_PlayerCharacter.CoinPickedUp` false _asbp_player_character_2)
            (`self.K2_DestroyActor`))))
      (:`then_1`
        (bind (_direction _slide) (`Timeline|Timeline_0`)
          (:`Update`
            (bind _returnvalue (+ _slide (`KismetMathLibrary.VInterpTo` (.location (`self.GetTransform`)) (`KismetMathLibrary.MakeVector` _returnvalue_x _returnvalue_y (+ _returnvalue_z 80.0)) (`GameplayStatics.GetWorldDeltaSeconds`) 15.0)))
            (`self.K2_SetActorLocation` _returnvalue)
            (`self.K2_SetActorTransform` (`KismetMathLibrary.MakeTransform` _returnvalue (struct) (0.4 0.4 0.4)))))))))

(fn `ReturnParent`
  (returns (Parent :type "/Game/Blueprints/Spawners/BP_SpawnerBase Object Reference"))
  (return (`self.ParentRef`)))

(fn `SetParent`
  (params (Parent :type "/Game/Blueprints/Spawners/BP_SpawnerBase Object Reference"))
  (returns (Return :type Boolean))
  (set `self.ParentRef` Parent)
  (return false))

(fn `UserConstructionScript`)