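; BP_Slowmo is a slow-motion pickup that flags the player character as slow-mo active for a timed period.
; On overlap, a DoOnce, reset if slow-mo is already active, gates setting the flag, a sound and a HUD animation.
; The pickup is moved away and hidden, then after a delay clears the flag and destroys itself.
; BeginPlay sets spin rates; time dilation is not applied here.
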(event `self.ReceiveBeginPlay`
  ;[1 1 1] Rotation
  (set `self.YawPerSecond` 200.0)
  (set `self.PitchPerSecond` 0.0))

(event `self.Pickup.OnComponentBeginOverlap`
  (params (OverlappedComponent :type "PrimitiveComponent Object Reference") (OtherActor :type "Actor Object Reference") (OtherComp :type "PrimitiveComponent Object Reference") (OtherBodyIndex :type Integer) (bFromSweep :type Boolean) (SweepResult :type "HitResult Structure (by ref)"))
  ;[1 1 1] Slow Mo Pickup
  (bind _asbp_player_character (cast `/Game/Characters/BP_PlayerCharacter` OtherActor))
  (if (`/Game/Characters/BP_PlayerCharacter.SlowMoActive` _asbp_player_character)
    (goto _label :!via `Reset`)
    (else
      (`/Engine/EditorBlueprintResources/StandardMacros.DoOnce` false :!label _label
        (:`Completed`
          (set `/Game/Characters/BP_PlayerCharacter.SlowMoActive` true _asbp_player_character)
          (`KismetSystemLibrary.PrintString` "SlowMo active" true true (struct :`R` 1.0 :`G` 0.224152 :`B` 0.043934 :`A` 1.0) 10.0)
          (`SceneComponent.K2_SetWorldLocation` (`self.Pickup`) (0.0 0.0 5000.0) false false)
          (`SceneComponent.SetVisibility` (`self.Pickup`) false false)
          (`GameplayStatics.PlaySound2D` null 1.0 1.0 0.0 null null)
          (`UserWidget.PlayAnimation` (`/Game/Characters/BP_PlayerCharacter.HUD` _asbp_player_character) null 0.0 1 "Forward" 1.0 false)
          (`KismetSystemLibrary.Delay` (`self.PickupTimer`))
          (bind _asbp_player_character_2 (cast `/Game/Characters/BP_PlayerCharacter` (`GameplayStatics.GetPlayerCharacter` 0)))
          (set `/Game/Characters/BP_PlayerCharacter.SlowMoActive` false _asbp_player_character_2)
          (`KismetSystemLibrary.PrintString` "SlowMo inactive" true true (struct :`R` 1.0 :`G` 0.224152 :`B` 0.043934 :`A` 1.0))
          (`self.K2_DestroyActor`))))))

(fn `UserConstructionScript`
  (`parent.UserConstructionScript`))