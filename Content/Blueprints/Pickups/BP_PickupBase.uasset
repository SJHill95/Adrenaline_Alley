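; Base pickup actor that spins in the world and removes itself when it overlaps an obstacle.
; Tick rotates the Pickup component in local pitch and yaw at per-second rates scaled by delta time.
; Any begin overlap on ObstacleTrigger destroys the actor, with no filtering in the graph.
; SetParent and ReturnParent store and expose a parent reference.
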(event `self.ReceiveTick`
  (params (DeltaSeconds :type "Float (single-precision)"))
  ;[1 1 1] Rotation
  (`SceneComponent.K2_AddLocalRotation` (`self.Pickup`) (`KismetMathLibrary.MakeRotator` 0.0 (* DeltaSeconds (`self.PitchPerSecond`)) (* DeltaSeconds (`self.YawPerSecond`))) false false))

(event `self.Obstacle Trigger.OnComponentBeginOverlap`
  (params (OverlappedComponent :type "PrimitiveComponent Object Reference") (OtherActor :type "Actor Object Reference") (OtherComp :type "PrimitiveComponent Object Reference") (OtherBodyIndex :type Integer) (bFromSweep :type Boolean) (SweepResult :type "HitResult Structure (by ref)"))
  ;[1 1 1] Destroy magnet if collides with obstacle
  (`self.K2_DestroyActor`))

(fn `ReturnParent`
  (returns (Parent :type "/Game/Blueprints/Spawners/BP_SpawnerBase Object Reference"))
  (return (`self.ParentRef`)))

(fn `SetParent`
  (params (Parent :type "/Game/Blueprints/Spawners/BP_SpawnerBase Object Reference"))
  (returns (Return :type Boolean))
  (set `self.ParentRef` Parent)
  (return false))

(fn `UserConstructionScript`)